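; BP_Mimic is a controllable pawn that sprouts NS_Mimic Niagara effects reaching toward nearby surfaces.
; Axis inputs drive movement relative to control rotation and mouse look.
; Each tick, UpdateTraces casts a debug-drawn visibility trace in a random direction within a forward cone, between two radii.
; Each hit, limited by a tiny cooldown, spawns a capsule-attached system fed the start point, impact point and normal.
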(event `InputAxis|Move Forward / Backward`
  (params (AxisValue :type "Float (single-precision)"))
  (bind (_returnvalue_roll _returnvalue_pitch _returnvalue_yaw) (`KismetMathLibrary.BreakRotator` (`self.GetControlRotation`)))
  (`self.AddMovementInput` (`KismetMathLibrary.GetForwardVector` (`KismetMathLibrary.MakeRotator` 0.0 0.0 _returnvalue_yaw)) AxisValue))

(event `self.ReceiveTick`
  (params (DeltaSeconds :type "Float (single-precision)"))
  (`self.Update Traces`))

(event `InputAxis|Move Right / Left`
  (params (AxisValue :type "Float (single-precision)"))
  (bind (_returnvalue_roll _returnvalue_pitch _returnvalue_yaw) (`KismetMathLibrary.BreakRotator` (`self.GetControlRotation`)))
  (`self.AddMovementInput` (`KismetMathLibrary.GetRightVector` (`KismetMathLibrary.MakeRotator` _returnvalue_roll 0.0 _returnvalue_yaw)) AxisValue))

(event `InputAxis|Look Up / Down Mouse`
  (params (AxisValue :type "Float (single-precision)"))
  (`self.AddControllerPitchInput` (* AxisValue -1.0)))

(event `InputAxis|Turn Right / Left Mouse`
  (params (AxisValue :type "Float (single-precision)"))
  (`self.AddControllerYawInput` AxisValue))

(fn `Update Traces`
  (bind _capsulecomponent (`self.CapsuleComponent`))
  (bind _randomdirection (`self.RandomDirection`))
  (bind _returnvalue (`SceneComponent.K2_GetComponentLocation` _capsulecomponent))
  (bind _returnvalue_2 (+ _returnvalue (* _randomdirection (`self.MinRadius`))))
  (set `self.TraceCooldown` 0.001)
  (if (> (- (`GameplayStatics.GetTimeSeconds`) (`self.LastTrace`)) (`self.TraceCooldown`))
    (set `self.RandomDirection` (`KismetMathLibrary.RandomUnitVectorInConeInDegrees` (`SceneComponent.GetForwardVector` _capsulecomponent) (`self.Cone Half Angle in Degrees`)))
    (bind (_outhit _returnvalue_3) (`KismetSystemLibrary.LineTraceSingle` :`Start` _returnvalue_2 :`End` (+ _returnvalue (* _randomdirection (`self.MaxRadius`))) :`TraceChannel` "TraceTypeQuery1" :`DrawDebugType` "ForDuration" :`DrawTime` 1.0))
    (if _returnvalue_3
      (set `self.LastTrace` (`GameplayStatics.GetTimeSeconds`))
      (bind _returnvalue_4 (`NiagaraFunctionLibrary.SpawnSystemAttached` "/Game/Art/Niagara/NS_Mimic.NS_Mimic" (`self.CapsuleComponent`) "None" (0.0 0.0 0.0) (struct) "KeepRelativeOffset"))
      (`NiagaraComponent.SetVariableVec3` _returnvalue_4 "StartPoint" _returnvalue_2)
      (bind (_bblockinghit _binitialoverlap _time _distance _location _impactpoint _normal _impactnormal) (`GameplayStatics.BreakHitResult` _outhit))
      (`NiagaraComponent.SetVariableVec3` _returnvalue_4 "EndPoint" _impactpoint)
      (`NiagaraComponent.SetVariableVec3` _returnvalue_4 "ImpactNormal" _impactnormal)
      (`PrimitiveComponent.SetCastShadow` _returnvalue_4 false))))

(fn `UserConstructionScript`)
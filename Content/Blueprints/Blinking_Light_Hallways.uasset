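; Blinking hallway light actor that makes its point light flicker endlessly from BeginPlay.
; Each cycle toggles the PointLight's visibility in two short flashes separated by brief random delays, then holds it dark for a longer random pause.
; The sequence is a chain of Delay nodes wired back to its start, with no Tick or Timeline.
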(event `self.ReceiveBeginPlay`
  (`SceneComponent.SetVisibility` (`self.PointLight`) false false :!label _label)
  (`KismetSystemLibrary.Delay` (`KismetMathLibrary.RandomFloatInRange` 0.2 0.5))
  (`SceneComponent.SetVisibility` (`self.PointLight`) true false)
  (`KismetSystemLibrary.Delay` (`KismetMathLibrary.RandomFloatInRange` 0.1 0.4))
  (`SceneComponent.SetVisibility` (`self.PointLight`) false false)
  (`KismetSystemLibrary.Delay` (`KismetMathLibrary.RandomFloatInRange` 0.2 0.5))
  (`SceneComponent.SetVisibility` (`self.PointLight`) true false)
  (`KismetSystemLibrary.Delay` (`KismetMathLibrary.RandomFloatInRange` 0.1 0.4))
  (`SceneComponent.SetVisibility` (`self.PointLight`) false false)
  (`KismetSystemLibrary.Delay` (`KismetMathLibrary.RandomFloatInRange` 1.5 5.0))
  (goto _label))

(fn `UserConstructionScript`)
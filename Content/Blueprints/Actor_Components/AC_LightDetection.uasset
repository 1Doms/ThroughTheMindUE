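; Actor component that measures light intensity through its owner's SceneCapture2D render target, storing a normalized Brightness value.
; Setup logic gives the capture its own render target copy; the intensity function reads the center pixel, weights RGB by luminance coefficients, then clamps and normalizes by MaxClamp.
; BeginPlay and Tick are empty, leaving both setup and brightness update disconnected, so neither runs.
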(event `self.ReceiveBeginPlay`
  ;[1 1 1] Find RT_Text
)

(event `self.ReceiveTick`
  (params (DeltaSeconds :type "Float (single-precision)"))
  ;[1 1 1] Update brightness value
  ;;[1 1 1] Get middle pixel
)

(fn `FC_GetPixelLightIntensity`
  (params (TextureRenderTarget :type "TextureRenderTarget2D Object Reference"))
  (bind _max_clamp (`self.Max_clamp`))
  (bind (_returnvalue_b _returnvalue_g _returnvalue_r) (`self.FC_GetPixelRenderTexture` TextureRenderTarget))
  (bind _output_get (set `self.Texture_brightness` (+ (* (`KismetMathLibrary.Conv_ByteToDouble` _returnvalue_b) 0.0722) (+ (* (`KismetMathLibrary.Conv_ByteToDouble` _returnvalue_g) 0.7152) (* (`KismetMathLibrary.Conv_ByteToDouble` _returnvalue_r) 0.2126)))))
  (set `self.Brightness` (/ (`KismetMathLibrary.FClamp` (`KismetMathLibrary.Conv_IntToDouble` (`KismetMathLibrary.Round` _output_get)) 0.0 _max_clamp) _max_clamp)))

(fn `FC_GetPixelRenderTexture`
  (params (TextureRenderTarget :type "TextureRenderTarget2D Object Reference"))
  (returns (ReturnValue_B :type Byte) (ReturnValue_G :type Byte) (ReturnValue_R :type Byte) (Current_render_texture :type "TextureRenderTarget2D Object Reference"))
  (bind _current_render_texture (`self.Current_render_texture`))
  (bind _returnvalue (`KismetRenderingLibrary.ReadRenderTargetPixel` TextureRenderTarget (/ (`TextureRenderTarget2D.SizeX` _current_render_texture) 2) (/ (`TextureRenderTarget2D.SizeY` _current_render_texture) 2)))
  (return (break `Color` _returnvalue) (`.G` (break `Color` _returnvalue)) (`.R` (break `Color` _returnvalue)) null))
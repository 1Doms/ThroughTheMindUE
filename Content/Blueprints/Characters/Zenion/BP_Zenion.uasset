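; BP_Zenion is an actor that reacts to being looked at by the player, sliding its mesh to a target point.
; It plays a sound on BeginPlay, then each Tick compares the player camera's forward vector with the direction to itself.
; The first dot product above the focus threshold rotates the mesh and opens a movement gate.
; The mesh then lerps from actor location to the Sphere component over a set duration, after which the gate closes.
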(event `self.ReceiveBeginPlay`
  (bind _asbp_player_character (cast `/Game/Blueprints/Characters/BP_PlayerCharacter` (`GameplayStatics.GetPlayerCharacter` 0)))
  (set `self.As BP Player Character` _asbp_player_character)
  (set `self.First Person Camera` (`/Game/Blueprints/Characters/BP_PlayerCharacter.FirstPersonCamera` (`self.As BP Player Character`)))
  (`GameplayStatics.SpawnSoundAtLocation` null (`self.K2_GetActorLocation`) (struct) 1.0 1.0 0.0 null null))

(event `self.ReceiveTick`
  (params (DeltaSeconds :type "Float (single-precision)"))
  (`|ExecutionSequence`
    (:`then_0`
      (`/Engine/EditorBlueprintResources/StandardMacros.Gate` false
        (:`Exit`
          (if (> (`KismetMathLibrary.Dot_VectorVector` (`KismetMathLibrary.GetDirectionUnitVector` (`SceneComponent.K2_GetComponentLocation` (`self.First Person Camera`)) (`self.K2_GetActorLocation`)) (`SceneComponent.GetForwardVector` (`self.First Person Camera`))) (`self.f_AngleFocus`))
            (`/Engine/EditorBlueprintResources/StandardMacros.DoOnce` false
              (:`Completed`
                (`self.CE_SetRotation`)
                (set `self.f_CurrentDuration` 0.0)
                (`self.CE_CanMove`)))))))
    (:`then_1`
      (`/Engine/EditorBlueprintResources/StandardMacros.Gate` true :!label _label
        (:`Exit`
          (`self.CE_MoveTo`))))))

(event `CE_CanMove`
  (goto _label :!via `Open`))

(event `CE_StopMove`
  (goto _label :!via `Close`))

(event `CE_MoveTo`
  (if (> (`self.f_CurrentDuration`) (`self.f_MoveDuration`))
    (`self.CE_MoveCompleted`)
    (else
      (set `self.f_CurrentDuration` (+ (`GameplayStatics.GetWorldDeltaSeconds`) (`self.f_CurrentDuration`)))
      (set `self.f_Alpha` (`KismetMathLibrary.NormalizeToRange` (`self.f_CurrentDuration`) 0.0 (`self.f_MoveDuration`)))
      (`SceneComponent.K2_SetWorldLocation` (`self.SkeletalMesh`) (`KismetMathLibrary.VLerp` (`self.K2_GetActorLocation`) (`SceneComponent.K2_GetComponentLocation` (`self.Sphere`)) (`self.f_Alpha`)) false false))))

(event `CE_MoveCompleted`
  (`self.CE_StopMove`))

(event `CE_SetRotation`
  (`SceneComponent.K2_SetWorldRotation` (`self.SkeletalMesh`) (`KismetMathLibrary.ComposeRotators` (`KismetMathLibrary.MakeRotFromX` (* (`SceneComponent.GetForwardVector` (`self.SkeletalMesh`)) -1.0)) (`SceneComponent.K2_GetComponentRotation` (`self.Sphere`))) false false))

(fn `UserConstructionScript`)
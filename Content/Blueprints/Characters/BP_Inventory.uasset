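; BP_Inventory is an inventory Blueprint that places items into slots, each slot being a BP_InventorySlot child actor.
; FC_AddItem asks FC_GetEmptySlot for a slot and sets the item on it, doing nothing if the item or slot is invalid.
; FC_GetEmptySlot walks all child actors, including descendants, and returns the first slot without a valid item.
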(event `self.ReceiveTick`
  (params (DeltaSeconds :type "Float (single-precision)")))

(fn `FC_AddItem`
  (params (Item :type "/Game/Blueprints/Interactible/Items/BP_MainItem Object Reference"))
  (locals (a_InventorySlot :type "/Game/Blueprints/Characters/BP_InventorySlot Object Reference") (a_Item :type "/Game/Blueprints/Interactible/Items/BP_MainItem Object Reference"))
  (`/Engine/EditorBlueprintResources/StandardMacros.IsValid` Item
    (:`Is Valid`
      (set `local.a_Item` Item)
      (bind _a_inventoryslot1 (`self.FC_GetEmptySlot`))
      (bind _output_get (set `local.a_InventorySlot` _a_inventoryslot1))
      (`/Engine/EditorBlueprintResources/StandardMacros.IsValid` _output_get
        (:`Is Valid`
          (`/Game/Blueprints/Characters/BP_InventorySlot.FC_SetItem` (`local.a_InventorySlot`) (`local.a_Item`)))))))

(fn `FC_GetEmptySlot`
  (returns (a_InventorySlot1 :type "/Game/Blueprints/Characters/BP_InventorySlot Object Reference"))
  (locals (a_InventorySlot :type "/Game/Blueprints/Characters/BP_InventorySlot Object Reference") (a_Item :type "SceneComponent Object Reference"))
  (for _array_element (`self.GetAllChildActors` true)
    (bind _asbp_inventory_slot (cast `/Game/Blueprints/Characters/BP_InventorySlot` _array_element))
    (bind _output_get (set `local.a_InventorySlot` _asbp_inventory_slot))
    (bind _output (`/Game/Blueprints/Characters/BP_InventorySlot.FC_GetItem` _output_get))
    (bind _output_get_2 (set `local.a_Item` _output))
    (`/Engine/EditorBlueprintResources/StandardMacros.IsValid` _output_get_2
      (:`Is Valid`
        (set `local.a_InventorySlot` null))
      (:`Is Not Valid`
        (break))))
  (return (`local.a_InventorySlot`)))

(fn `UserConstructionScript`)
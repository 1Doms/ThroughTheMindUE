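; AI-moved transition pawn that travels to the alpha AI character, then blends the player's view onto it.
; On begin play it finds the alpha, starts a transition sound and shows the finisher widget.
; Tick reissues the move, while a DoOnce-gated delay loop periodically halts movement with a flash and sound before restoring high speed.
; On arrival it clears the sound and widget, makes the alpha visible and destroys itself.
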(event `self.ReceiveBeginPlay`
  (`self.FC_Init`))

(event `self.ReceiveTick`
  (params (DeltaSeconds :type "Float (single-precision)"))
  (bind _alpha_ref (`self.Alpha_ref`))
  (bind _charactermovement (`self.CharacterMovement`))
  (`|AIMoveTo` self (0.0 0.0 0.0) (`self.Alpha_ref`)
    (:`then`
      (`/Engine/EditorBlueprintResources/StandardMacros.DoOnce` false :!label _label
        (:`Completed`
          (`KismetSystemLibrary.Delay` 2.0)
          (set `CharacterMovementComponent.MaxWalkSpeed` 0.0 _charactermovement)
          (`/Game/UI/Widgets/WBP_Finisher.Flash_event` (`self.Widget_ref`))
          (`GameplayStatics.PlaySound2D` "/Game/Audio/Sounds/Alpha/Flash_Cue.Flash_Cue" 1.0 1.0 0.0 null null)
          (`KismetSystemLibrary.Delay` 1.0)
          (set `CharacterMovementComponent.MaxWalkSpeed` 1500.0 _charactermovement)
          (goto _label :!via `Reset`))))
    (:`OnSuccess`
      (`PlayerController.SetViewTargetWithBlend` (`GameplayStatics.GetPlayerController` 0) _alpha_ref 0.0 "VTBlend_EaseInOut" 0.0 false)
      (`AudioComponent.Stop` (`self.Transition_sound_ref`))
      (`Widget.RemoveFromParent` (`self.Widget_ref`))
      (set `/Game/Blueprints/AI/Blueprints/BP_AI_character_alpha.Visible?` true _alpha_ref)
      (`self.K2_DestroyActor`))))

(fn `FC_Init`
  (bind _returnvalue (`GameplayStatics.GetActorOfClass` "/Game/Blueprints/AI/Blueprints/BP_AI_character_alpha.BP_AI_character_alpha_C"))
  (`/Engine/EditorBlueprintResources/StandardMacros.IsValid` _returnvalue
    (:`Is Valid`
      (set `self.Alpha_ref` _returnvalue)
      (bind _returnvalue_2 (`GameplayStatics.SpawnSound2D` "/Game/Audio/Sounds/Alpha/Transition_flash_Cue.Transition_flash_Cue" 1.0 1.0 0.0 null))
      (set `self.Transition_sound_ref` _returnvalue_2)
      (bind _returnvalue_3 (`|CreateWidget` "/Game/UI/Widgets/WBP_Finisher.WBP_Finisher_C"))
      (bind _output_get (set `self.Widget_ref` _returnvalue_3))
      (`UserWidget.AddToViewport` _output_get 0))))

(fn `UserConstructionScript`)
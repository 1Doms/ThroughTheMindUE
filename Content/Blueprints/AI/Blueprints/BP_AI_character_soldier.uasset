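; Soldier AI character that patrols an assigned spline, reacts to sight and sound, and shoots Alpha or Player targets.
; Perception events write target, hearing and death state to the Blackboard and trigger voice lines.
; DetectionScore scales walk speed, burst size, timing and spread of hitscan fire, which damages only the player and reports noise.
; Velocity-timed traces spawn footstep impacts, and the construction script flags missing patrol splines.
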(event Custom|Steps
  (bind _returnvalue (Transformation|GetActorLocation))
  (bind _charactermovement (Variables|Character|GetCharacterMovement))
  (bind _velocity (Variables|/Script/Engine.MovementComponent|GetVelocity _charactermovement))
  (bind _returnvalue_2 (Math|Vector|VectorLength _velocity))
  (if (> _returnvalue_2 3e+01)
    (Utilities|FlowControl|Delay (Math|Float|MapRangeClamped _returnvalue_2 0.0 5e+02 0.75 0.25))
    (bind (_outhit _returnvalue_3) (Collision|LineTraceByChannel _returnvalue (- _returnvalue "0.000000,0.000000,200.000000") "TraceTypeQuery1" false 0 "None"))
    (if _returnvalue_3
      (Game|SpawnActorfromClass "/Game/VFX/Impact/BP_impact.BP_impact_C" (Math|Transform|MakeTransform (.Location (Collision|BreakHitResult _outhit)) "0, 0, 0" "1.000000,1.000000,1.000000") "AlwaysSpawn" "MultiplyWithRoot" 0 _outhit "NewEnumerator3" self "/Game/Audio/Sounds/SA_Generic.SA_Generic" 0))))

(event Custom|VoiceIdle
  (bind _soldier_voice (Variables|Default|GetSoldier_Voice))
  (if (not (Variables|Default|GetAlpha?))
    (if (not (Variables|Default|GetPlayer?))
      (Utilities|FlowControl|Delay (Math|Random|RandomFloatinRange 5.0 25.0))
      (Audio|Components|Audio|SetSound _soldier_voice "/Game/Audio/Sounds/Soldiers/Voices/Soldier_idle_voice_3_Cue.Soldier_idle_voice_3_Cue")
      (Audio|Components|Audio|Play _soldier_voice 0.0))))

(event Custom|Damages
  (Variables|Default|SetDead? true)
  (AI|Components|Blackboard|SetValueasBool (AI|GetBlackboard 0) (Utilities|Name|MakeLiteralName "Dead?") true)
  (Components|DestroyComponent (Variables|Default|GetAIPerception)))

(event EventBeginPlay
  (|CallParentFunction)
  (AI|Components|Blackboard|SetValueasObject (AI|GetBlackboard 0) (Utilities|Name|MakeLiteralName "Spline") (Variables|Spline|GetSpline_ref))
  (AI|Components|Blackboard|SetValueasBool (AI|GetBlackboard 0) (Utilities|Name|MakeLiteralName "isSplineLooping") (Variables|Spline|GetisSplineLooping)))

(event Collision|EventActorBeginOverlap
  (params (OtherActor :type Actor%20Object%20Reference))
  (|CallParentFunction OtherActor) ; This node is disabled and will not be called.\nDrag off pins to build functionality.
)

(event EventHeardHostileSound
  (params (Heard_location :type Vector :default "0, 0, 0"))
  (bind _returnvalue (AI|GetBlackboard 0))
  ;[0.007497 0 1] Modify key variables of BB_alpha
  (AI|Components|Blackboard|SetValueasBool _returnvalue (Utilities|Name|MakeLiteralName "Heard?") true)
  (AI|Components|Blackboard|SetValueasVector _returnvalue (Utilities|Name|MakeLiteralName "Heard_location") Heard_location))

(event EventSuccesfullSensed
  (params (Actor_ref :type Actor%20Object%20Reference))
  (bind _soldier_voice (Variables|Default|GetSoldier_Voice))
  ;[0.007497 0 1] Modify key variables of BB_alpha
  (Audio|Components|Audio|SetSound _soldier_voice "/Game/Audio/Sounds/Soldiers/Voices/Soldier_contact_voice_3_Cue.Soldier_contact_voice_3_Cue")
  (Audio|Components|Audio|Play _soldier_voice 0.0))

(event EventNotSensed
  (params (Actor_removed :type Actor%20Object%20Reference))
  ;[0.007497 0 1] Modify key variables of BB_alpha
  (if (Utilities|Array|IsEmpty (Variables|Default|GetArray_of_actors_detected))
    (Variables|Default|SetAlpha? false)
    (Variables|Default|SetPlayer? false)
    (AI|Components|Blackboard|SetValueasBool (AI|GetBlackboard 0) (Utilities|Name|MakeLiteralName "Alpha?") false)
    (AI|Components|Blackboard|SetValueasBool (AI|GetBlackboard 0) (Utilities|Name|MakeLiteralName "Player?") false)))

(event EventTargetSet
  (params (Target_ref :type Actor%20Object%20Reference) (Target_Location :type Vector :default "0, 0, 0"))
  (bind _returnvalue (Actor|ActorHasTag Target_ref "Alpha"))
  (bind _returnvalue_2 (Actor|ActorHasTag Target_ref "Player"))
  (bind _soldier_voice (Variables|Default|GetSoldier_Voice))
  ;[0.007497 0 1] Modify key variables of BB_alpha
  (Variables|Default|SetTarget%20Location Target_Location)
  (AI|Components|Blackboard|SetValueasObject (AI|GetBlackboard 0) (Utilities|Name|MakeLiteralName "Target_reference") Target_ref)
  (AI|Components|Blackboard|SetValueasBool (AI|GetBlackboard 0) (Utilities|Name|MakeLiteralName "Alpha?") _returnvalue)
  (Variables|Default|SetAlpha? _returnvalue)
  (AI|Components|Blackboard|SetValueasBool (AI|GetBlackboard 0) (Utilities|Name|MakeLiteralName "Player?") _returnvalue_2)
  (Variables|Default|SetPlayer? _returnvalue_2)
  (Audio|Components|Audio|SetSound _soldier_voice "/Game/Audio/Sounds/Soldiers/Voices/Soldier_Shoot_voice_3_Cue.Soldier_Shoot_voice_3_Cue")
  (Audio|Components|Audio|Play _soldier_voice 0.0)
  (if (Class|KismetMathLibrary|XORBoolean (Variables|Default|GetAlpha?) (Variables|Default|GetPlayer?))
    (if (not (Variables|Default|GetDead?))
      (Utilities|Shoot))))

(event EventSetRoamingRaddius
  ;[0.007497 0 1] Modify key variables of BB_alpha
  (AI|Components|Blackboard|SetValueasFloat (AI|GetBlackboard 0) (Utilities|Name|MakeLiteralName "Roaming_Radius") (Variables|Default|GetRoaming_radius)))

(event EventTick
  (params (DeltaSeconds :type Float%20%28single-precision%29))
  (|CallParentFunction DeltaSeconds)
  (bind _output_get (Variables|Default|SetScore_detection (Variables|Default|GetDetection_Score)))
  (Variables|Default|SetAiming _output_get)
  (CallFunction|VoiceIdle)
  (CallFunction|Steps)
  (Variables|/Script/Engine.CharacterMovementComponent|SetMaxWalkSpeed (Variables|Character|GetCharacterMovement) (Math|Float|MapRangeClamped (Variables|Default|GetScore_detection) 0.0 1.0 (Variables|Default|GetMin_Speed) (Variables|Default|GetMax_Speed)))
  (AI|Components|Blackboard|SetValueasFloat (AI|GetBlackboard 0) (Utilities|Name|MakeLiteralName "Precision") (Math|Float|MapRangeClamped (Variables|Default|GetScore_detection) 0.0 1.0 5.0 0.0))
  (Class|BlackboardComponent|SetValueasInt (AI|GetBlackboard 0) (Utilities|Name|MakeLiteralName "Firerate") (Math|Float|Truncate (Math|Float|MapRangeClamped (Variables|Default|GetScore_detection) 0.0 1.0 1.0 15.0))))

(event EventStopHeardHostileSound
  ;[0.007497 0 1] Modify key variables of BB_alpha
  (AI|Components|Blackboard|SetValueasBool (AI|GetBlackboard 0) (Utilities|Name|MakeLiteralName "Heard?") false))

(event Input|KeyboardEvents|DebugKeyE
  (params (Key :type Key%20Structure :default "None") (ActionValue :type Input%20Action%20Value%20Structure)))

(fn ConstructionScript
  (bind _spline_ (Variables|Default|GetSpline?))
  (|CallParentFunction)
  (Utilities|IsValid (Variables|Spline|GetSpline_ref)
    (:Is%20Valid
      (Rendering|Components|TextRender|SetText _spline_ (Utilities|Text|MakeLiteralText "Patrol spline assigned"))
      (Rendering|Components|TextRender|SetTextRenderColor _spline_ (Math|Color|MakeColor 0 255 0 255)))
    (:Is%20Not%20Valid
      (Rendering|Components|TextRender|SetText _spline_ (Utilities|Text|MakeLiteralText "! Patrol spline unassigned !"))
      (Rendering|Components|TextRender|SetTextRenderColor _spline_ (Math|Color|MakeColor 0 0 255 255)))))

(fn FCShoot
  (params (ConeHalfAngleInDegrees :type Float%20%28single-precision%29))
  (bind _returnvalue (Transformation|GetActorLocation))
  (Variables|Default|SetFire? true)
  (Audio|PlaySoundatLocation "/Game/Audio/Sounds/Soldiers/Soldier_shoot_Cue.Soldier_shoot_Cue" _returnvalue "0, 0, 0" 1.0 1.0 0.0 "/Game/Audio/Sounds/SA_Generic.SA_Generic" 0 0 0)
  (bind _outhit (Collision|LineTraceByChannel (Transformation|GetActorLocation) (+ _returnvalue (* (Math|Random|RandomUnitVectorinConeinDegrees (Transformation|GetActorForwardVector) ConeHalfAngleInDegrees) 1e+04) "0.000000,0.000000,250.000000") "TraceTypeQuery2" false (Utilities|Array|MakeArray self) "None" true "(R=1.000000,G=0.000000,B=0.000000,A=1.000000)" "(R=0.000000,G=1.000000,B=0.000000,A=1.000000)" 1.0))
  (Niagara|SpawnSystematLocation "/Game/VFX/Muzzle/NS_MuzzleDefault.NS_MuzzleDefault" (Transformation|GetWorldLocation (Variables|Default|GetMuzzleSocket)))
  (Class|AISenseHearing|ReportNoiseEvent (Transformation|GetActorLocation) 1.0 self 0.0 "Soldier")
  (bind _asbp_player_character (Utilities|Casting|CastToBP_PlayerCharacter (.HitActor (Collision|BreakHitResult _outhit)))
    (:then
      (Default|Damages _asbp_player_character))
    (:CastFailed
      (Game|SpawnActorfromClass :Class "/Game/VFX/Impact/BP_impact.BP_impact_C" :SpawnTransform (Math|Transform|MakeTransform (.Location (Collision|BreakHitResult _outhit)) "0, 0, 0" "1.000000,1.000000,1.000000") :CollisionHandlingOverride "AlwaysSpawn" :TransformScaleMethod "MultiplyWithRoot" :Impact_Owner self :Attenuation%20Settings "/Game/Audio/Sounds/SA_Generic.SA_Generic" :Instigator 0))))
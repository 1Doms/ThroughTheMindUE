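; Base AI character with stealth-style detection of players and other AI, exposing empty events for children to react to targets and hostile sounds.
; AI Perception tracks seen actors lacking its own tag and reports hostile sounds.
; Each tick scores seen actors by distance, view angle and light-detected brightness, choosing the highest above a threshold as target.
; That score drives walk speed, while velocity scales acceleration, braking and eased turn rate.
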(event `Heard_hostile_sound`
  (params (Heard_location :type "Vector Structure")))

(event `Stop_heard_hostile_sound`)

(event `Succesfull_sensed`
  (params (Actor_ref :type "Actor Object Reference")))

(event `Not_sensed`
  (params (Actor_removed :type "Actor Object Reference")))

(event `self.AIPerception.OnPerceptionUpdated`
  (params (UpdatedActors :type "Array of Actor Object Reference (by ref)"))
  (bind _target (`self.Target`))
  (bind _array_of_actors_detected (`self.Array_of_actors_detected`))
  ;[1 1 1] get all actor seen
  (for _array_element UpdatedActors
    (bind _info (`AIPerceptionComponent.GetActorsPerception` (`self.AIPerception`) _array_element))
    (bind (_target_2 _lastsensedstimuli) (break `ActorPerceptionBlueprintInfo` _info))
    (bind _output_get (set `self.Target` _target_2))
    (if (not (`self.ActorHasTag` _output_get (`|GetArrayItem` (`self.Tags`))))
      (for (_array_element_2 _array_index) _lastsensedstimuli
        (switch `int` _array_index
          (:`0`
            (bind (_age _expirationage _strength _stimuluslocation _receiverlocation _tag _bsuccessfullysensed) (break `AIStimulus` _array_element_2))
            (if _bsuccessfullysensed
              (`KismetArrayLibrary.Array_Add` _array_of_actors_detected _target)
              (`KismetArrayLibrary.Array_Add` (`self.Array_of_detection_score`))
              ;[0.9743 0 1] Debug
              (`KismetSystemLibrary.PrintString` (`KismetSystemLibrary.GetDisplayName` _target) true false (struct :`G` 1.0 :`B` 0.006319 :`A` 1.0) 1.0)
              (`self.Succesfull_sensed` _target)
              (else
                (`KismetArrayLibrary.Array_RemoveItem` _array_of_actors_detected _target)
                (`KismetArrayLibrary.Array_Remove` (`self.Array_of_detection_score`) (+ (`KismetArrayLibrary.Array_Find` _array_of_actors_detected _target) 1))
                (`KismetSystemLibrary.PrintString` (`KismetSystemLibrary.GetDisplayName` _target) true false (struct :`R` 1.0 :`B` 0.095176 :`A` 1.0) 1.0)
                (`self.Not_sensed` _target :!label _label))))
          (:`1`
            (if (== _tag "None")
              _
              (elif (!= _tag (`KismetStringLibrary.Conv_StringToName` (`KismetStringLibrary.Concat_StrStr` (`KismetStringLibrary.Conv_NameToString` (`|GetArrayItem` (`self.Tags`))) "Sound")))
                (if _bsuccessfullysensed
                  (`self.Heard_hostile_sound` _stimuluslocation)
                  (else
                    (`self.Stop_heard_hostile_sound`)))))))))))

(event `Hide`
  (goto _label))

(event `Set_Roaming_Raddius`)

(event `self.ReceiveBeginPlay`
  (`self.Set_Roaming_Raddius`))

(event `self.ReceiveTick`
  (params (DeltaSeconds :type "Float (single-precision)"))
  (bind _array_of_actors_detected (`self.Array_of_actors_detected`))
  (bind _array_of_detection_score (`self.Array_of_detection_score`))
  (bind (_indexofmaxvalue _maxvalue) (`KismetMathLibrary.MaxOfFloatArray` (`self.Array_of_detection_score`)))
  (`self.Acceleration_Deceleration`)
  (`self.Rotation`)
  (`self.Tick_child` DeltaSeconds)
  (if (`KismetArrayLibrary.Array_IsEmpty` _array_of_detection_score)
    (set `self.Detection_Score` 0.0)
    (else
      (set `self.Detection_Score` (`.MaxValue` (`KismetMathLibrary.MaxOfFloatArray` _array_of_detection_score)))))
  (`self.Modify_Speed`)
  (`KismetSystemLibrary.DelayUntilNextTick`)
  (bind _asbp_light_detection (cast `/Game/Blueprints/AI/Blueprints/BP_LightDetection` (`ChildActorComponent.ChildActor` (`self.BP_LightDetection`))))
  (set `self.Self_brightness` (`/Game/Blueprints/AI/Blueprints/BP_LightDetection.BP_LightDetection_Brightness` _asbp_light_detection))
  (if (not (`KismetArrayLibrary.Array_IsEmpty` _array_of_actors_detected))
    (for (_array_element _array_index) _array_of_actors_detected
      (`self.Calcul_detection_score` _array_element _array_index))
    (if (> _maxvalue 0.2)
      (bind _output_get (set `self.Choosen_target` (`|GetArrayItem` (`self.Array_of_actors_detected`) _indexofmaxvalue)))
      (`self.Target_set` _output_get (`self.K2_GetActorLocation` _output_get))
      (else
        (set `self.Target` (`self.Choosen_target`))
        (`self.Hide`)
        (set `self.Choosen_target` null)))))

(event `Target_set`
  (params (Target_ref :type "Actor Object Reference") (Target_Location :type "Vector Structure")))

(event `Tick_child`
  (params (Delta_seconds :type "Float (double-precision)")))

(event `Modify_Speed`
  (bind _charactermovement (`self.CharacterMovement`))
  (bind _min_speed (`self.Min_Speed`))
  (if (`KismetSystemLibrary.IsValid` (`self.Choosen_target`))
    (set `CharacterMovementComponent.MaxWalkSpeed` (`KismetMathLibrary.MapRangeClamped` (`.MaxValue` (`KismetMathLibrary.MaxOfFloatArray` (`self.Array_of_detection_score`))) 0.0 1.0 _min_speed (`self.Max_Speed`)) _charactermovement)
    (else
      (set `CharacterMovementComponent.MaxWalkSpeed` _min_speed _charactermovement))))

(event `Rotation`
  (bind _charactermovement (`self.CharacterMovement`))
  (bind _returnvalue (`CharacterMovementComponent.GetLastUpdateRotation` _charactermovement))
  (bind (_rotationrate_roll _rotationrate_pitch _rotationrate_yaw) (`KismetMathLibrary.BreakRotator` (`CharacterMovementComponent.RotationRate` _charactermovement)))
  (`|ExecutionSequence`
    (:`then_0`
      (`/Engine/EditorBlueprintResources/StandardMacros.DoOnce` false :!label _label_2
        (:`Completed`
          (set `self.Last_rotation` _returnvalue)
          (set `self.Ease_alpha` 0.0))))
    (:`then_1`
      (if (not (== _returnvalue (`self.Last_rotation`) :`ErrorTolerance` 1.0))
        (set `self.Ease_alpha` (+ (`GameplayStatics.GetWorldDeltaSeconds`) (/ (`self.Ease_alpha`) 1.05)))
        (set `CharacterMovementComponent.RotationRate` (`KismetMathLibrary.MakeRotator` 0.0 0.0 (`|EaseFunction` "ExpoInOut" (`self.Ease_alpha`) _rotationrate_yaw (`KismetMathLibrary.MapRangeClamped` (`KismetMathLibrary.VSize` (`MovementComponent.Velocity` _charactermovement)) 0.0 1000.0 (`self.Min_rotation_Speed`) (`self.Max_Rotation_Speed`)))) _charactermovement)
        (if (>= (`self.Ease_alpha`) 1.0)
          (goto _label_2 :!via `Reset`))))))

(event `Acceleration_Deceleration`
  (bind _charactermovement (`self.CharacterMovement`))
  (bind _returnvalue (`KismetMathLibrary.VSize` (`MovementComponent.Velocity` (`self.CharacterMovement`))))
  (set `CharacterMovementComponent.MaxAcceleration` (`KismetMathLibrary.MapRangeClamped` _returnvalue 0.0 1000.0 (`self.Min_acceleration`) (`self.Max_Acceleration`)) _charactermovement)
  (set `CharacterMovementComponent.BrakingDecelerationWalking` (`KismetMathLibrary.MapRangeClamped` _returnvalue 0.0 1000.0 (`self.Min_Deceleration`) (`self.Max_Deceleration`)) _charactermovement))

(fn `Angle_between_two_vectors`
  (params (`Vector 1` :type "Vector Structure") (`Vector 2` :type "Vector Structure"))
  (returns (Angle :type "Float (double-precision)"))
  (return (`KismetMathLibrary.DegAcos` (`KismetMathLibrary.Dot_VectorVector` (`KismetMathLibrary.Normal` `Vector 1`) (`KismetMathLibrary.Normal` `Vector 2`)))))

(fn `UserConstructionScript`)
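; Alpha AI character Blueprint that reports sensing results to its blackboard and plays a help sound at random intervals.
; Sensing events set or clear the target flag, clearing only when no detected actors remain.
; Other events write the target reference, location and roaming radius to blackboard keys.
; TickChild uses a random Delay to space out the attached sound and a debug "Hello" print.
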(event `self.ReceiveActorBeginOverlap`
  (params (OtherActor :type "Actor Object Reference"))
  (`parent.ReceiveActorBeginOverlap` OtherActor))

(event `self.Tick_child`
  (params (Delta_seconds :type "Float (double-precision)"))
  (`KismetSystemLibrary.Delay` (`KismetMathLibrary.RandomFloatInRange` 1.0 10.0))
  (bind _returnvalue (`GameplayStatics.SpawnSoundAttached` "/Game/Sounds/Sounds/Alpha/Help_cue.Help_cue" (`self.CapsuleComponent`) "None" (`self.K2_GetActorLocation`) (struct) "SnapToTargetIncludingScale" true 1.0 1.0 0.0 "/Game/Sounds/Sounds/SA_test.SA_test" null))
  (`AudioComponent.Play` _returnvalue 0.0)
  (`KismetSystemLibrary.PrintString` "Hello"))

(event `self.Succesfull_sensed`
  (params (Actor_ref :type "Actor Object Reference"))
  ;[0.007497 0 1] Modify key variables of BB_alpha
  (`BlackboardComponent.SetValueAsBool` (`AIBlueprintHelperLibrary.GetBlackboard` null) "Target?" true))

(event `self.Not_sensed`
  (params (Actor_removed :type "Actor Object Reference"))
  ;[0.007497 0 1] Modify key variables of BB_alpha
  (if (`KismetArrayLibrary.Array_IsEmpty` (`self.Array_of_actors_detected`))
    (`BlackboardComponent.SetValueAsBool` (`AIBlueprintHelperLibrary.GetBlackboard` null) "Target?" false)))

(event `self.Target_set`
  (params (Target_ref :type "Actor Object Reference") (Target_Location :type "Vector Structure"))
  (bind _returnvalue (`AIBlueprintHelperLibrary.GetBlackboard` null))
  ;[0.007497 0 1] Modify key variables of BB_alpha
  (`BlackboardComponent.SetValueAsObject` _returnvalue "Target_reference" Target_ref)
  (`BlackboardComponent.SetValueAsVector` _returnvalue "Target_Location" Target_Location))

(event `self.Set_Roaming_Raddius`
  ;[0.007497 0 1] Modify key variables of BB_alpha
  (`BlackboardComponent.SetValueAsFloat` (`AIBlueprintHelperLibrary.GetBlackboard` null) "Roaming_Radius" (`self.Roaming_radius`)))

(fn `UserConstructionScript`
  (`parent.UserConstructionScript`))
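; Short-lived tentacle actor that snaps to its owner and anchors a tentacle effect to nearby geometry.
; On BeginPlay it traces in a random cone along its arrow, destroying itself on a miss or spawning the effect between itself and the hit point.
; Physics-simulating hits receive a distance-scaled impulse.
; Tick updates the effect's start and destroys both once the anchor is over half the maximum distance away.
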(event `self.ReceiveBeginPlay`
  (bind _returnvalue (`self.K2_GetActorLocation`))
  (bind _arrow (`self.Arrow`))
  (bind _tantacle_ref (`self.Tantacle_ref`))
  (`self.K2_AttachToActor` (`self.GetOwner`) "None" "SnapToTarget" "SnapToTarget" "KeepRelative")
  (bind (_outhit _returnvalue_2) (`KismetSystemLibrary.LineTraceSingle` :`Start` (`self.K2_GetActorLocation`) :`End` (+ (* (`KismetMathLibrary.RandomUnitVectorInConeInDegrees` (`SceneComponent.GetForwardVector` _arrow) (`self.Tantacle_angle_spawn`)) (`self.Tantacle_max_distance`)) (`SceneComponent.K2_GetComponentLocation` _arrow)) :`TraceChannel` "TraceTypeQuery1" :`DrawTime` 1.0))
  (if _returnvalue_2
    (bind (_bblockinghit _binitialoverlap _time _distance _location _impactpoint _normal _impactnormal _physmat _hitactor _hitcomponent) (`GameplayStatics.BreakHitResult` _outhit))
    (if (`SceneComponent.IsSimulatingPhysics` _hitcomponent "None")
      (`PrimitiveComponent.AddImpulseAtLocation` _hitcomponent (* (`KismetMathLibrary.Normal` (`KismetMathLibrary.GetDirectionUnitVector` (`self.End_location`) (`self.K2_GetActorLocation`))) _distance) _impactpoint "None"))
    (bind _returnvalue_3 (`NiagaraFunctionLibrary.SpawnSystemAtLocation` (`self.Tantacle_system`) _returnvalue (struct) (1.0 1.0 1.0) false))
    (set `self.Tantacle_ref` _returnvalue_3)
    (set `self.Distance_to_keep` _distance)
    (`FXSystemComponent.SetVectorParameter` _tantacle_ref "Tantacle_Start" _returnvalue)
    (`FXSystemComponent.SetVectorParameter` _tantacle_ref "Tantacle_End" _location)
    (set `self.End_location` _location)
    (set `self.Tantacle_exist` true)
    (else
      (`self.K2_DestroyActor`))))

(event `self.ReceiveTick`
  (params (DeltaSeconds :type "Float (single-precision)"))
  (if (`self.Tantacle_exist`)
    (`FXSystemComponent.SetVectorParameter` (`self.Tantacle_ref`) "Tantacle_Start" (`self.K2_GetActorLocation`))
    (if (> (`KismetMathLibrary.Vector_Distance` (`self.End_location`) (`self.K2_GetActorLocation`)) (/ (`self.Tantacle_max_distance`) 2.0))
      (`ActorComponent.K2_DestroyComponent` (`self.Tantacle_ref`))
      (`self.K2_DestroyActor`))))

(fn `UserConstructionScript`)
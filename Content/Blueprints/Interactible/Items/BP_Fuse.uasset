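; Carryable fuse item that the player grabs and holds in front of the first-person camera while the interaction input is held.
; Grabbing uses the player's PhysicsHandle and slows the player, and dropping releases it and restores speed.
; A gated Tick pulses the RectLight with a sine wave from first grab until CE_PutToHolder, which also disables physics and collision.
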(event `self.ReceiveTick`
  (params (DeltaSeconds :type "Float (single-precision)"))
  (`/Engine/EditorBlueprintResources/StandardMacros.Gate` true :!label _label
    (:`Exit`
      (bind _output_get (set `self.f_CurrentLightTime` (+ (`self.f_CurrentLightTime`) (* (`GameplayStatics.GetWorldDeltaSeconds`) (`self.f_LightSpeedMultiplier`)))))
      (`LightComponent.SetIntensity` (`self.RectLight`) (`KismetMathLibrary.Lerp` 0.0 3500.0 (`KismetMathLibrary.Abs` (`KismetMathLibrary.Sin` _output_get)))))))

(event `CE_Shine`
  (goto _label :!via `Open`))

(event `self.ReceiveBeginPlay`
  (`self.CE_Init`))

(event `CE_Unshine`
  (goto _label :!via `Close`))

(event `/Game/Blueprints/Interactible/BPI_Interaction.Interaction`
  (params (InputState :type "/Game/Blueprints/Characters/E_InputState Enum" :default "NewEnumerator0") (PlayerRef :type "/Game/Blueprints/Characters/BP_PlayerCharacter Object Reference") (Item :type "/Game/Blueprints/Interactible/BP_MainInteractible Object Reference"))
  (set `self.Input State` InputState)
  (switch `/Game/Blueprints/Characters/E_InputState` (`self.Input State`)
    (:`NewEnumerator0`
      (`self.CE_GrabItem` :!label _label_2))
    (:`NewEnumerator2`
      (goto _label_2))
    (:`NewEnumerator3`
      (`self.CE_DropItem` :!label _label_3))
    (:`NewEnumerator4`
      (goto _label_3))))

(event `CE_SetPlayerSpeed`
  (params (`b_GrabFuse?` :type Boolean))
  (bind _player_ref (`self.Player Ref`))
  (bind _f_defaultspeed (`/Game/Blueprints/Characters/BP_PlayerCharacter.f_DefaultSpeed` (`self.Player Ref`)))
  (if `b_GrabFuse?`
    (set `self.f_PlayerDefault Speed` _f_defaultspeed)
    (set `/Game/Blueprints/Characters/BP_PlayerCharacter.f_DefaultSpeed` (* _f_defaultspeed (`self.f_SlowMultiplier`)) (`self.Player Ref`))
    (else
      (set `/Game/Blueprints/Characters/BP_PlayerCharacter.f_DefaultSpeed` (`self.f_PlayerDefault Speed`) (`self.Player Ref`))))
  (`/Game/Blueprints/Characters/BP_PlayerCharacter.CE_ChangeState` _player_ref (`/Game/Blueprints/Characters/BP_PlayerCharacter.E_PlayerState` _player_ref)))

(event `self.CE_GrabItem`
  (bind _staticmesh (`self.StaticMesh`))
  (`self.CE_Init`)
  (`/Engine/EditorBlueprintResources/StandardMacros.IsValid` (`PhysicsHandleComponent.GetGrabbedComponent` (`self.Physics Handle`))
    (:`Is Valid`
      (`self.FC SetItemLocation`))
    (:`Is Not Valid`
      (`self.CE_SetPlayerSpeed` true)
      (set `/Game/Blueprints/Characters/BP_PlayerCharacter.ShouldGrip` true (`self.Player Ref`))
      (`PrimitiveComponent.SetSimulatePhysics` (`self.StaticMesh`) true)
      (`PrimitiveComponent.SetCollisionEnabled` (`self.Sphere`) "NoCollision")
      (`PrimitiveComponent.SetCollisionEnabled` (`self.StaticMesh`) "QueryAndPhysics")
      (`self.K2_SetActorLocationAndRotation` (`SceneComponent.K2_GetComponentLocation` _staticmesh) (`SceneComponent.K2_GetComponentRotation` _staticmesh) false true)
      (`PhysicsHandleComponent.GrabComponentAtLocationWithRotation` (`self.Physics Handle`) (`self.StaticMesh`) "None" (`self.K2_GetActorLocation`) (`self.K2_GetActorRotation`))
      (`SceneComponent.SetVisibility` (`self.RectLight`) true false)
      (`self.CE_Shine`))))

(event `self.CE_DropItem`
  (`PrimitiveComponent.SetCollisionEnabled` (`self.Sphere`) "QueryOnly")
  (`PrimitiveComponent.SetCollisionEnabled` (`self.StaticMesh`) "QueryAndPhysics")
  (`/Engine/EditorBlueprintResources/StandardMacros.IsValid` (`PhysicsHandleComponent.GetGrabbedComponent` (`self.Physics Handle`))
    (:`Is Valid`
      (`PhysicsHandleComponent.ReleaseComponent` (`self.Physics Handle`)))
    (:`Is Not Valid`
      (`PrimitiveComponent.SetSimulatePhysics` (`self.StaticMesh`) true)))
  (`self.CE_SetPlayerSpeed` false))

(event `CE_PutToHolder`
  (`self.CE_Init`)
  (`self.CE_DropItem`)
  (`PrimitiveComponent.SetSimulatePhysics` (`self.StaticMesh`) false)
  (`PrimitiveComponent.SetCollisionEnabled` (`self.Sphere`) "NoCollision")
  (`PrimitiveComponent.SetCollisionEnabled` (`self.StaticMesh`) "NoCollision")
  (`SceneComponent.SetVisibility` (`self.RectLight`) false false)
  (`self.CE_Unshine`))

(event `CE_Init`
  (bind _asbp_player_character (cast `/Game/Blueprints/Characters/BP_PlayerCharacter` (`GameplayStatics.GetPlayerCharacter` 0)))
  (set `self.Player Ref` _asbp_player_character)
  (set `self.Physics Handle` (`/Game/Blueprints/Characters/BP_PlayerCharacter.PhysicsHandle` (`self.Player Ref`))))

(fn `FC SetItemLocation`
  (bind _firstpersoncamera (`/Game/Blueprints/Characters/BP_PlayerCharacter.FirstPersonCamera` (`self.Player Ref`)))
  (bind _firstpersoncamera_2 (`/Game/Blueprints/Characters/BP_PlayerCharacter.FirstPersonCamera` (`self.Player Ref`)))
  (`PhysicsHandleComponent.SetTargetLocationAndRotation` (`self.Physics Handle`) (+ (`SceneComponent.K2_GetComponentLocation` _firstpersoncamera_2) (* (`SceneComponent.GetForwardVector` _firstpersoncamera_2) 50.0) (* (`SceneComponent.GetUpVector` _firstpersoncamera_2) -25.0)) (`KismetMathLibrary.MakeRotFromYZ` (`SceneComponent.GetForwardVector` _firstpersoncamera) (`SceneComponent.GetUpVector` _firstpersoncamera))))

(fn `UserConstructionScript`
  (`parent.UserConstructionScript`))
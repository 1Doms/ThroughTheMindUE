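; BP_MainItem is an interactible item that the player can pick up, with an empty Use event as a hook for item behavior.
; On Interaction it asks BP_PlayerCharacter whether it can add an item, then passes itself to FCAddItem and destroys its actor.
; IA_Use calls Use on both Started and Completed, while the code adding the IMC_Use mapping context is disconnected and never runs.
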(event `/Game/Blueprints/Interactible/BPI_Interaction.Interaction`
  (`|ExecutionSequence`
    (:`then_0`
      (bind _asbp_player_character (cast `/Game/Blueprints/Characters/BP_PlayerCharacter` (`GameplayStatics.GetPlayerCharacter` 0)))
      (bind _returnvalue (`/Game/Blueprints/Characters/BP_PlayerCharacter.FC_CanAddItem?` _asbp_player_character))
      (if _returnvalue
        (`/Game/Blueprints/Characters/BP_PlayerCharacter.FC_AddItem` _asbp_player_character self)
        (`self.K2_DestroyActor`)))))

(event `EnhancedInput|/Game/Blueprints/Characters/Input/Actions/IA_Use`
  (params (ActionValue :type Boolean) (ElapsedSeconds :type "Float (double-precision)") (TriggeredSeconds :type "Float (double-precision)") (InputAction :type "InputAction Object Reference" :default "/Game/Blueprints/Characters/Input/Actions/IA_Use.IA_Use"))
  (:`Started`
    (`self.Use` :!label _label))
  (:`Completed`
    (goto _label)))

(event `Use`)

(fn `UserConstructionScript`
  (`parent.UserConstructionScript`))
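; BP_Bullet is a physics projectile that spawns a list of Niagara effects after launch or on impact.
; Shoot launches the sphere forward with a velocity-change impulse, then waits a configurable delay before triggering effects unless ActivateOnHit is set.
; In hit mode, effects fire once, or on every hit above a speed threshold with MultipleHitActivation.
; FC_Niagara spawns each system either attached to the sphere or at its location.
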(event `Shoot`
  (bind _sphere1 (`self.Sphere1`))
  ;[1 1 1] Activate children effects
  ;;[1 1 1] Shoot
  (`PrimitiveComponent.AddImpulse` _sphere1 (* (`SceneComponent.GetForwardVector` _sphere1) (`self.f_ShootForce`)) "None" true)
  (`KismetSystemLibrary.Delay` (`self.DelayBeforeActivation`))
  (`self.ActivationWithDelay`))

(event `ActivationWithDelay`
  ;[1 1 1] Activate children effects
  (if (not (`self.ActivateOnHit?`))
    (`self.FC_Niagara` (`self.Attached to Bullet?`))))

(event `ActivationWithHit`
  ;[1 1 1] Activate children effects
  (if (`self.ActivateOnHit?`)
    (`self.FC_Niagara` (`self.Attached to Bullet?`))))

(event `self.Sphere1.OnComponentHit`
  (params (HitComponent :type "PrimitiveComponent Object Reference") (OtherActor :type "Actor Object Reference") (OtherComp :type "PrimitiveComponent Object Reference") (NormalImpulse :type "Vector Structure") (Hit :type "HitResult Structure (by ref)"))
  ;[1 1 1] Activate children effects
  (if (`self.MultipleHitActivation?`)
    (if (> (`KismetMathLibrary.VSize` (`SceneComponent.GetComponentVelocity` (`self.Sphere1`))) (`self.BulletEffectSleep`))
      (`self.ActivationWithHit` :!label _label))
    (else
      (`/Engine/EditorBlueprintResources/StandardMacros.DoOnce` false
        (:`Completed`
          (goto _label))))))

(fn `FC_Niagara`
  (params (`AttachedToBullet?` :type Boolean))
  (bind _sphere1 (`self.Sphere1`))
  (for _array_element (`self.Niagara`)
    (if `AttachedToBullet?`
      (`NiagaraFunctionLibrary.SpawnSystemAttached` _array_element _sphere1 "None" (0.0 0.0 0.0) (struct) "SnapToTargetIncludingScale" true)
      (else
        (`NiagaraFunctionLibrary.SpawnSystemAtLocation` _array_element (`SceneComponent.K2_GetComponentLocation` _sphere1))))))

(fn `UserConstructionScript`
  (`parent.UserConstructionScript`))
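; Flare gun pickup that the player carries in first person to fire light, smoke or EMP bullets.
; Interaction attaches it to the GripPoint socket, flags the player as armed, adds the use input context and disables pickup collision.
; Use toggles aiming by adding or removing the shoot mapping context.
; Shooting spawns the selected bullet at the Socket component and launches it, with debug keys switching type.
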(event `self.ReceiveBeginPlay`)

(event `/Game/Blueprints/Interactible/BPI_Interaction.Interaction`
  (params (InputState :type "/Game/Blueprints/Characters/E_InputState Enum" :default "NewEnumerator0") (Item :type "/Game/Blueprints/Interactible/BP_MainInteractible Object Reference"))
  (`|ExecutionSequence`
    (:`then_0`
      (bind _output_get (`self.FC_GetPlayerCharacter`))
      (`self.K2_AttachToComponent` (`/Game/Blueprints/Characters/BP_PlayerCharacter.FirstPersonMesh` _output_get) "GripPoint" "SnapToTarget" "SnapToTarget" "SnapToTarget")
      (set `/Game/Blueprints/Characters/BP_PlayerCharacter.b_HasRifle` true (`self.As BP Player Character`)))
    (:`then_1`
      (bind _asplayer_controller (cast `PlayerController` (`Pawn.GetController` (`GameplayStatics.GetPlayerCharacter` 0))))
      (bind _returnvalue (pcsubsystem `EnhancedInputLocalPlayerSubsystem` _asplayer_controller))
      (`/Engine/EditorBlueprintResources/StandardMacros.IsValid` _returnvalue
        (:`Is Valid`
          (`EnhancedInputSubsystemInterface.AddMappingContext` _returnvalue "/Game/Blueprints/Characters/Input/IMC_Use.IMC_Use" 3 (struct)))))
    (:`then_2`
      (`PrimitiveComponent.SetCollisionEnabled` (`self.Sphere_0`) "NoCollision"))))

(event `self.Use`
  (bind _asplayer_controller (cast `PlayerController` (`Pawn.GetController` (`GameplayStatics.GetPlayerCharacter` 0))))
  (bind _returnvalue (pcsubsystem `EnhancedInputLocalPlayerSubsystem` _asplayer_controller))
  (`/Engine/EditorBlueprintResources/StandardMacros.IsValid` _returnvalue
    (:`Is Valid`
      (if (`.ReturnValue` (`EnhancedInputSubsystemInterface.HasMappingContext` _returnvalue "/Game/Blueprints/Characters/Input/IMC_Shoot.IMC_Shoot"))
        (`EnhancedInputSubsystemInterface.RemoveMappingContext` _returnvalue "/Game/Blueprints/Characters/Input/IMC_Shoot.IMC_Shoot" (struct))
        (bind _output_get (`self.FC_GetPlayerCharacter`))
        (set `/Game/Blueprints/Characters/BP_PlayerCharacter.b_IsAiming` false _output_get)
        (else
          (`EnhancedInputSubsystemInterface.AddMappingContext` _returnvalue "/Game/Blueprints/Characters/Input/IMC_Shoot.IMC_Shoot" 3 (struct))
          (bind _output_get_2 (`self.FC_GetPlayerCharacter`))
          (set `/Game/Blueprints/Characters/BP_PlayerCharacter.b_IsAiming` true _output_get_2))))))

(event `EnhancedInput|/Game/Blueprints/Characters/Input/Actions/IA_Shoot`
  (params (ActionValue :type Boolean) (ElapsedSeconds :type "Float (double-precision)") (TriggeredSeconds :type "Float (double-precision)") (InputAction :type "InputAction Object Reference" :default "/Game/Blueprints/Characters/Input/Actions/IA_Shoot.IA_Shoot"))
  (bind _socket (`self.Socket`))
  (:`Started`
    (bind _returnvalue (`|SpawnActorFromClass` (select `int` (`self.Index_debug_bullet`) :`0` "/Game/Blueprints/Interactible/Items/Bullets/BP_LightBullet.BP_LightBullet_C" :`1` "/Game/Blueprints/Interactible/Items/Bullets/BP_SmokeBullet.BP_SmokeBullet_C" :`2` "/Game/Blueprints/Interactible/Items/Bullets/BP_EMPBullet.BP_EMPBullet_C" :!type "Actor Class Reference") (`KismetMathLibrary.MakeTransform` (`SceneComponent.K2_GetComponentLocation` _socket) (`SceneComponent.K2_GetComponentRotation` _socket)) "AlwaysSpawn" "MultiplyWithRoot" null null))
    (bind _asbp_bullet (cast `/Game/Blueprints/Interactible/Items/Bullets/BP_Bullet` _returnvalue))
    (`/Game/Blueprints/Interactible/Items/Bullets/BP_Bullet.Shoot` _asbp_bullet)))

(event `Key|F`
  (params (Key :type "Key Structure"))
  (:`Pressed`
    (set `self.Index_debug_bullet` 0)
    (`KismetSystemLibrary.PrintString` "Light")))

(event `Key|G`
  (params (Key :type "Key Structure"))
  (:`Pressed`
    (set `self.Index_debug_bullet` 1)
    (`KismetSystemLibrary.PrintString` "SMoke")))

(event `Key|H`
  (params (Key :type "Key Structure"))
  (:`Pressed`
    (set `self.Index_debug_bullet` 2)
    (`KismetSystemLibrary.PrintString` "EMP")))

(fn `FC_GetPlayerCharacter`
  (returns (Output_Get :type "/Game/Blueprints/Characters/BP_PlayerCharacter Object Reference"))
  (bind _asbp_player_character (cast `/Game/Blueprints/Characters/BP_PlayerCharacter` (`GameplayStatics.GetPlayerCharacter` 0)))
  (bind _output_get (set `self.As BP Player Character` _asbp_player_character))
  (return _output_get))

(fn `UserConstructionScript`
  (`parent.UserConstructionScript`))
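; BP_Screen is an environment screen actor whose glow can be switched on or off through the CELight custom event.
; CELight takes a boolean and creates a new dynamic material instance from the Screen component's first material slot on every call.
; It sets that instance's emissive intensity and color to a pale green glow or to black, then applies it back to the Screen.
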(event `self.CE_Light`
  (params (b_Light :type Boolean))
  (bind _screen (`self.Screen`))
  (bind _screen_2 (`self.Screen`))
  (if b_Light
    (bind _returnvalue (`PrimitiveComponent.CreateDynamicMaterialInstance` _screen 0 (`PrimitiveComponent.GetMaterial` _screen 0) "None"))
    (set `self.Mat` _returnvalue)
    (`MaterialInstanceDynamic.SetScalarParameterValue` (`self.Mat`) "Emissive Intensity" 3.0)
    (`MaterialInstanceDynamic.SetVectorParameterValue` (`self.Mat`) "Emissive_Color" (struct :`R` 0.784314 :`G` 1.0 :`B` 0.615686 :`A` 1.0))
    (`PrimitiveComponent.SetMaterial` (`self.Screen`) 0 (`self.Mat`))
    (else
      (bind _returnvalue_2 (`PrimitiveComponent.CreateDynamicMaterialInstance` _screen_2 0 (`PrimitiveComponent.GetMaterial` _screen_2 0) "None"))
      (set `self.Mat` _returnvalue_2)
      (`MaterialInstanceDynamic.SetScalarParameterValue` (`self.Mat`) "Emissive Intensity" 0.0)
      (`MaterialInstanceDynamic.SetVectorParameterValue` (`self.Mat`) "Emissive_Color" (struct :`A` 1.0))
      (`PrimitiveComponent.SetMaterial` (`self.Screen`) 0 (`self.Mat`)))))

(fn `UserConstructionScript`
  (`parent.UserConstructionScript`))
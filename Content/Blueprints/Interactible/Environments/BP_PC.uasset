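; BP_PC is an interactible environment computer that switches its screen UI on and off.
; Its activation and deactivation events, plus their Child variants, get the WBP_PC widget from the WBPWatch component and call Activate with true or false.
; The Blueprint holds no other logic, as BeginPlay, overlap and Tick are disabled.
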(event `self.Child_Desactivated`
  (bind _aswbp_pc (cast `/Game/UI/Widgets/WBP_PC` (`WidgetComponent.GetWidget` (`self.WBP_Watch`)) :!label _label))
  (`/Game/UI/Widgets/WBP_PC.Activate` _aswbp_pc false))

(event `/Game/Blueprints/Interactible/BPI_Interaction.Desactived`
  (goto _label))

(event `/Game/Blueprints/Interactible/BPI_Interaction.Activated`
  (bind _aswbp_pc (cast `/Game/UI/Widgets/WBP_PC` (`WidgetComponent.GetWidget` (`self.WBP_Watch`)) :!label _label_2))
  (`/Game/UI/Widgets/WBP_PC.Activate` _aswbp_pc true))

(event `self.Child_Activated`
  (goto _label_2))

(fn `UserConstructionScript`
  (`parent.UserConstructionScript`))
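; Base Blueprint for environment interactibles that can be activated, deactivated or temporarily hit by an EMP.
; Activation events call empty child hook functions for subclasses, but are ignored while the EMP flag is set.
; The EMP event sets that flag, calls its own hook and clears the flag after the given duration.
; Linked actors register uniquely, and a currently unused check sets the on state false if any is off.
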(event `self.ReceiveTick`
  (params (DeltaSeconds :type "Float (single-precision)"))
  (`parent.ReceiveTick` DeltaSeconds))

(event `/Game/Blueprints/Interactible/BPI_Interaction.Activated`
  (if (not (`self.EMP?`))
    (`self.Child_Activated`)))

(event `/Game/Blueprints/Interactible/BPI_Interaction.Desactived`
  (if (not (`self.EMP?`))
    (`self.Child_Desactivated`)))

(event `/Game/Blueprints/Interactible/Items/Bullets/EMP/IEMP.EMP`
  (params (EMPDuration :type "Float (double-precision)"))
  (set `self.EMP?` true)
  (`self.Child_EMP`)
  (`KismetSystemLibrary.Delay` EMPDuration)
  (set `self.EMP?` false))

(event `CE_AddActorLinked`
  (params (Actor :type "/Game/Blueprints/Interactible/Triggers/BP_MainTriggers Object Reference (by ref)"))
  (`KismetArrayLibrary.Array_AddUnique` (`self.ActorLinked`) Actor))

(fn `Child_Activated`)

(fn `Child_Desactivated`)

(fn `Child_EMP`)

(fn `FC_GetActorIsOn`
  (returns (b_IsOn1 :type Boolean))
  (locals (b_IsOn :type Boolean :default true))
  (for _array_element (`self.ActorLinked`)
    (if (not (`/Game/Blueprints/Interactible/Triggers/BP_MainTriggers.b_IsOn` _array_element))
      (set `local.b_IsOn` false)
      (break)))
  (return (`local.b_IsOn`)))

(fn `UserConstructionScript`
  (`parent.UserConstructionScript`))
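; Switchable lab ceiling light that pairs a rect light with an emissive mesh material.
; Activation, light on/off and EMP events funnel into CE_TurnLight, which sets visibility and refreshes the emissive glow through a dynamic material instance.
; Switching on also plays an attenuated sound and reports a "Light"-tagged noise event at the lamp.
; The construction script applies ActivateOnPlay so the initial state shows in the editor.
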(event `self.ReceiveBeginPlay`
  (set `self.b_isActive?` (`SceneComponent.bVisible` (`self.RectLight`)))
  (`self.CE_RefreshLight`))

(event `/Game/Blueprints/Interactible/BPI_Interaction.Activated`
  (`self.CE_TurnLight` true :!label _label))

(event `self.Child_Activated`
  (goto _label))

(event `LightOn`
  (goto _label))

(event `self.Child_Desactivated`
  (`self.CE_TurnLight` false :!label _label_2))

(event `LightOff`
  (goto _label_2))

(event `/Game/Blueprints/Interactible/BPI_Interaction.Desactived`
  (goto _label_2))

(event `self.Child_EMP`
  (set `self.b_isOverlap` false)
  (`self.CE_TurnLight` false))

(event `CE_TurnLight`
  (params (bNewVisibility :type Boolean))
  (set `self.b_IsOn` bNewVisibility)
  (`SceneComponent.SetVisibility` (`self.RectLight`) (`self.b_IsOn`) false)
  (`self.CE_RefreshLight`)
  (if (`self.b_IsOn`)
    (`self.CE_SoundAtLamp` (`self.SoundLightOn`))))

(event `Set_all_light_intensity`
  (bind _outactors (`GameplayStatics.GetAllActorsOfClass` "/Game/Blueprints/Interactible/Environments/BP_Light.BP_Light_C"))
  (for _ _outactors
    (`LightComponent.SetIntensity` (`self.RectLight`) (`LightComponentBase.Intensity` (`self.RectLight`)))))

(event `CE_RefreshLight`
  (bind _returnvalue (`PrimitiveComponent.CreateDynamicMaterialInstance` (`self.SM_CeilingLight`) 1 "/Game/Environments/Props/Materials/Instances/MI_EmissiveCeilingLight.MI_EmissiveCeilingLight" "None"))
  (`MaterialInstanceDynamic.SetScalarParameterValue` _returnvalue "Emissive Intensity" (select `bool` (`SceneComponent.IsVisible` (`self.RectLight`)) :`true` 2.0 :!type "Float (single-precision)")))

(event `CE_SoundAtLamp`
  (params (Sound :type "SoundBase Object Reference"))
  (`GameplayStatics.PlaySoundAtLocation` Sound (`SceneComponent.K2_GetComponentLocation` (`self.SM_CeilingLight`)) (struct) 1.0 1.0 0.0 "/Game/Audio/Sound_attenuation/SA_Mid.SA_Mid" null null null)
  (`AISense_Hearing.ReportNoiseEvent` (`SceneComponent.K2_GetComponentLocation` (`self.SM_CeilingLight`)) 1.0 null 0.0 "Light"))

(fn `UserConstructionScript`
  (`SceneComponent.SetVisibility` (`self.RectLight`) (`self.ActivateOnPlay`) false)
  (`self.CE_RefreshLight`))
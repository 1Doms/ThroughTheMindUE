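; BP_Vent is an interactible environment vent whose mesh starts simulating physics when activated.
; Three activation events share one path that enables physics and plays a start sound, while deactivation does nothing.
; While simulating, Tick compares angular velocity to SoundThreshold and, after a random delay, plays a swing sound with volume scaled by spin speed.
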(event `self.ReceiveBeginPlay`
  (`parent.ReceiveBeginPlay`))

(event `self.ReceiveTick`
  (params (DeltaSeconds :type "Float (single-precision)"))
  (bind _staticmesh (`self.StaticMesh`))
  (bind _returnvalue (`KismetMathLibrary.VSize` (`PrimitiveComponent.GetPhysicsAngularVelocityInDegrees` _staticmesh "None")))
  (`parent.ReceiveTick` DeltaSeconds)
  (if (`SceneComponent.IsSimulatingPhysics` _staticmesh "None")
    (if (> _returnvalue (`self.SoundThreshold`))
      (`KismetSystemLibrary.Delay` (`KismetMathLibrary.RandomFloat`))
      (`GameplayStatics.PlaySoundAtLocation` "/Game/Audio/Sounds/Vents/vent_swing_1_Cue.vent_swing_1_Cue" (`SceneComponent.K2_GetComponentLocation` (`self.StaticMesh`)) (struct) (`KismetMathLibrary.MapRangeClamped` _returnvalue 0.0 180.0 0.5 3.0) 1.0 0.0 "/Game/Audio/Sound_attenuation/SA_Generic.SA_Generic" null null null))))

(event `self.Child_Activated`
  (`PrimitiveComponent.SetSimulatePhysics` (`self.StaticMesh`) true :!label _label)
  (`GameplayStatics.PlaySoundAtLocation` "/Game/Audio/Sounds/Vents/Vent_start_Cue.Vent_start_Cue" (`SceneComponent.K2_GetComponentLocation` (`self.StaticMesh`)) (struct) 1.0 1.0 0.0 "/Game/Audio/Sound_attenuation/SA_Long.SA_Long" null null null))

(event `/Game/Blueprints/Interactible/BPI_Interaction.Activated`
  (goto _label))

(event `self.CE_EnviroActivated`
  (goto _label))

(event `self.Child_Desactivated`)

(fn `UserConstructionScript`
  (`parent.UserConstructionScript`))
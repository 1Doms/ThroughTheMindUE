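; BP_TSM_Appear is an environment interactible that makes a static mesh appear when activated, then removes itself.
; BeginPlay uniformly scales the Static component by FScale.
; CEEnviroActivated waits SpawnDelay, then assigns SpawnMesh and plays a 2D sound, and destroys the actor once LifeTime elapses.
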(event `self.ReceiveBeginPlay`
  (`SceneComponent.SetRelativeScale3D` (`self.Static`) (* (1.0 1.0 1.0) (`self.f_Scale`))))

(event `self.CE_EnviroActivated`
  (`KismetSystemLibrary.Delay` (`self.SpawnDelay`))
  (`|ExecutionSequence`
    (:`then_0`
      (`StaticMeshComponent.SetStaticMesh` (`self.Static`) (`self.SpawnMesh`))
      (`KismetSystemLibrary.Delay` (`self.LifeTime`))
      (`self.K2_DestroyActor`))
    (:`then_1`
      (`GameplayStatics.PlaySound2D` (`self.Sound`) 1.0 1.0 0.0 null null))))

(fn `UserConstructionScript`
  (`parent.UserConstructionScript`))
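; BP_BigDesk is an environment desk actor with built-in lighting that can be switched on or off.
; Its CELight event takes a boolean, toggles three spotlights and sets the mesh's second material slot to glow warm or go dark to match.
; Each call creates a new dynamic material instance from the current material; the file contains no caller or other active logic.
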(event `self.CE_Light`
  (params (b_Light :type Boolean))
  (bind _staticmesh (`self.StaticMesh`))
  (bind _staticmesh_2 (`self.StaticMesh`))
  (if b_Light
    (`SceneComponent.SetVisibility` (`self.SpotLight`) true false)
    (`SceneComponent.SetVisibility` (`self.SpotLight1`) true false)
    (`SceneComponent.SetVisibility` (`self.SpotLight2`) true false)
    (bind _returnvalue (`PrimitiveComponent.CreateDynamicMaterialInstance` _staticmesh_2 1 (`PrimitiveComponent.GetMaterial` _staticmesh_2 1) "None"))
    (set `self.Mat` _returnvalue)
    (`MaterialInstanceDynamic.SetScalarParameterValue` (`self.Mat`) "Emissive Intensity" 2.0)
    (`MaterialInstanceDynamic.SetVectorParameterValue` (`self.Mat`) "Emissive_Color" (struct :`R` 1.0 :`G` 0.733333 :`B` 0.337255 :`A` 1.0))
    (`PrimitiveComponent.SetMaterial` (`self.StaticMesh`) 1 (`self.Mat`))
    (else
      (`SceneComponent.SetVisibility` (`self.SpotLight`) false false)
      (`SceneComponent.SetVisibility` (`self.SpotLight1`) false false)
      (`SceneComponent.SetVisibility` (`self.SpotLight2`) false false)
      (bind _returnvalue_2 (`PrimitiveComponent.CreateDynamicMaterialInstance` _staticmesh 1 (`PrimitiveComponent.GetMaterial` _staticmesh 1) "None"))
      (set `self.Mat` _returnvalue_2)
      (`MaterialInstanceDynamic.SetScalarParameterValue` (`self.Mat`) "Emissive Intensity" 0.0)
      (`MaterialInstanceDynamic.SetVectorParameterValue` (`self.Mat`) "Emissive_Color" (struct :`A` 1.0))
      (`PrimitiveComponent.SetMaterial` (`self.StaticMesh`) 1 (`self.Mat`)))))

(fn `UserConstructionScript`
  (`parent.UserConstructionScript`))
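; BP_Door is an interactable environment door that opens and closes by hiding and showing its static mesh.
; Activated alternates between OpenDoor and CloseDoor through a FlipFlop, while Desactived always calls CloseDoor without resetting that FlipFlop.
; Both functions set BIsOpen and mesh visibility only, with no movement or collision change.
; DoorType switching, a Gate and a relative-location move are unconnected leftovers that never run.
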(event `/Game/Blueprints/Interactible/BPI_Interaction.Activated`
  (`/Engine/EditorBlueprintResources/StandardMacros.FlipFlop`
    (:`A`
      (`self.Open Door`))
    (:`B`
      (`self.Close Door` :!label _label))))

(event `/Game/Blueprints/Interactible/BPI_Interaction.Desactived`
  (goto _label))

(fn `Close Door`
  (set `self.b_isOpen?` false)
  (`SceneComponent.SetVisibility` (`self.StaticMesh`) true false))

(fn `Open Door`
  (set `self.b_isOpen?` true)
  (`SceneComponent.SetVisibility` (`self.StaticMesh`) false false))

(fn `UserConstructionScript`
  (`parent.UserConstructionScript`))
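; Environment trigger actor that starts scenario events on linked TSM actors when it receives an activation or deactivation event.
; BIsActivated selects which event responds: activated when true, deactivated when false, each gated by a DoOnce.
; Both paths share a delay of FSpawnDelay, then loop through ActorLink, cast each entry to TSM and call CEScenarioActivated.
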(event `self.CE_EnviroDesactivated`
  (if (not (`self.b_IsActivated`))
    (`/Engine/EditorBlueprintResources/StandardMacros.DoOnce` false
      (:`Completed`
        (`KismetSystemLibrary.Delay` (`self.f_SpawnDelay`) :!label _label)
        (if (`KismetArrayLibrary.Array_IsValidIndex` (`self.ActorLink`))
          (for _array_element (`self.ActorLink`)
            (bind _astsm (cast `/Game/Blueprints/Interactible/Environments/Scenario/TSM` _array_element))
            (`/Game/Blueprints/Interactible/Environments/Scenario/TSM.CE_ScenarioActivated` _astsm)))))))

(event `self.CE_EnviroActivated`
  (if (`self.b_IsActivated`)
    (`/Engine/EditorBlueprintResources/StandardMacros.DoOnce` false
      (:`Completed`
        (goto _label)))))

(fn `UserConstructionScript`
  (`parent.UserConstructionScript`))
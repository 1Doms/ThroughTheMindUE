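; BP_RedLight02 is a red ceiling light environment prop that can be switched on or off.
; The CELight event creates a dynamic material instance from the mesh's slot 1 material, sets its emissive to glowing red or dark, also assigns it to slot 0, and toggles the spotlight's visibility to match.
; The construction script calls CELight with ActivateOnPlay, so the initial state is applied at construction rather than in BeginPlay.
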(event `self.CE_Light`
  (params (b_Light :type Boolean))
  (bind _sm_ceilinglightlab (`self.SM_CeilingLightLab`))
  (bind _sm_ceilinglightlab_2 (`self.SM_CeilingLightLab`))
  (if b_Light
    (bind _returnvalue (`PrimitiveComponent.CreateDynamicMaterialInstance` _sm_ceilinglightlab 1 (`PrimitiveComponent.GetMaterial` _sm_ceilinglightlab 1) "None"))
    (set `self.Mat` _returnvalue)
    (`MaterialInstanceDynamic.SetScalarParameterValue` (`self.Mat`) "Emissive Intensity" 3.0)
    (`MaterialInstanceDynamic.SetVectorParameterValue` (`self.Mat`) "Emissive_Color" (struct :`R` 1.0 :`A` 1.0))
    (`PrimitiveComponent.SetMaterial` (`self.SM_CeilingLightLab`) 0 (`self.Mat`))
    (`SceneComponent.SetVisibility` (`self.SpotLight1`) true false)
    (else
      (bind _returnvalue_2 (`PrimitiveComponent.CreateDynamicMaterialInstance` _sm_ceilinglightlab_2 1 (`PrimitiveComponent.GetMaterial` _sm_ceilinglightlab_2 1) "None"))
      (set `self.Mat` _returnvalue_2)
      (`MaterialInstanceDynamic.SetScalarParameterValue` (`self.Mat`) "Emissive Intensity" 0.0)
      (`MaterialInstanceDynamic.SetVectorParameterValue` (`self.Mat`) "Emissive_Color" (struct :`A` 1.0))
      (`PrimitiveComponent.SetMaterial` (`self.SM_CeilingLightLab`) 0 (`self.Mat`))
      (`SceneComponent.SetVisibility` (`self.SpotLight1`) false false))))

(fn `UserConstructionScript`
  (`self.CE_Light` (`self.ActivateOnPlay`)))
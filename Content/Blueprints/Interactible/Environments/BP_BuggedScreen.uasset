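; BP_BuggedScreen is an environment screen prop that switches between a glitchy noise display and a black, unlit state.
; CELight takes a boolean, sets the mesh's second material slot to MI_Noise or MI_Black, and toggles the RectLight to match.
; The Construction Script applies the ActivateOnPlay flag through CELight.
; Each switch also stores a dynamic material instance in Mat, though SetMaterial immediately replaces it on the mesh.
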(event `self.CE_Light`
  (params (b_Light :type Boolean))
  (bind _staticmesh (`self.StaticMesh`))
  (bind _staticmesh_2 (`self.StaticMesh`))
  (if b_Light
    (bind _returnvalue (`PrimitiveComponent.CreateDynamicMaterialInstance` _staticmesh 1 (`PrimitiveComponent.GetMaterial` _staticmesh 1) "None"))
    (set `self.Mat` _returnvalue)
    (`PrimitiveComponent.SetMaterial` (`self.StaticMesh`) 1 "/Game/Environments/Props/Materials/Instances/MI_Noise.MI_Noise")
    (`SceneComponent.SetVisibility` (`self.RectLight`) true false)
    (else
      (bind _returnvalue_2 (`PrimitiveComponent.CreateDynamicMaterialInstance` _staticmesh_2 1 (`PrimitiveComponent.GetMaterial` _staticmesh_2 1) "None"))
      (set `self.Mat` _returnvalue_2)
      (`PrimitiveComponent.SetMaterial` (`self.StaticMesh`) 1 "/Game/Environments/Props/Materials/Instances/MI_Black.MI_Black")
      (`SceneComponent.SetVisibility` (`self.RectLight`) false false))))

(fn `UserConstructionScript`
  (`self.CE_Light` (`self.ActivateOnPlay`)))
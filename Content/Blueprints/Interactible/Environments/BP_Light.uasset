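; BP_Light is an interactable environment lamp that switches a spotlight on and off through activation, light and EMP events.
; Toggling sets spotlight visibility and drives an emissive scalar on the lamp's dynamic material to match.
; Switching on plays an attenuated sound at the lamp and reports a "Light"-tagged noise event.
; A separate event copies this light's intensity to every BP_Light in the level.
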(event `self.ReceiveBeginPlay`
  (set `self.b_isActive?` (`SceneComponent.bVisible` (`self.SpotLight`)))
  (`self.CE_RefreshLight`))

(event `/Game/Blueprints/Interactible/BPI_Interaction.Activated`
  (`self.CE_TurnLight` true :!label _label))

(event `self.Child_Activated`
  (goto _label))

(event `LightOn`
  (goto _label))

(event `self.Child_Desactivated`
  (`self.CE_TurnLight` false :!label _label_2))

(event `LightOff`
  (goto _label_2))

(event `/Game/Blueprints/Interactible/BPI_Interaction.Desactived`
  (goto _label_2))

(event `self.Child_EMP`
  (set `self.b_isOverlap` false)
  (`self.CE_TurnLight` false))

(event `CE_TurnLight`
  (params (bNewVisibility :type Boolean))
  (set `self.b_IsOn` bNewVisibility)
  (`SceneComponent.SetVisibility` (`self.SpotLight`) (`self.b_IsOn`) false)
  (`self.CE_RefreshLight`)
  (if (`self.b_IsOn`)
    (`self.CE_SoundAtLamp` (`self.SoundLightOn`))))

(event `Set_all_light_intensity`
  (bind _outactors (`GameplayStatics.GetAllActorsOfClass` "BP_Light_C"))
  (for _array_element _outactors
    (`LightComponent.SetIntensity` (`/Game/Blueprints/Interactible/Environments/BP_Light.SpotLight` _array_element) (`LightComponentBase.Intensity` (`self.SpotLight`)))))

(event `CE_RefreshLight`
  (bind _returnvalue (`PrimitiveComponent.CreateDynamicMaterialInstance` (`self.Lamp`) 0 "/Game/Environments/Props/Materials/Instances/MI_Emissive3.MI_Emissive3" "None"))
  (`MaterialInstanceDynamic.SetScalarParameterValue` _returnvalue "B" (select `bool` (`SceneComponent.IsVisible` (`self.SpotLight`)) :`true` 2.0 :!type "Float (single-precision)")))

(event `CE_SoundAtLamp`
  (params (Sound :type "SoundBase Object Reference"))
  (`GameplayStatics.PlaySoundAtLocation` Sound (`SceneComponent.K2_GetComponentLocation` (`self.Lamp`)) (struct) 1.0 1.0 0.0 "/Game/Audio/Sound_attenuation/SA_Long.SA_Long" null null null)
  (`AISense_Hearing.ReportNoiseEvent` (`SceneComponent.K2_GetComponentLocation` (`self.Lamp`)) 1.0 null 0.0 "Light"))

(fn `UserConstructionScript`)
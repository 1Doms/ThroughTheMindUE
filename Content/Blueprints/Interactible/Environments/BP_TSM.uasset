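; BP_TSM is an environment interactible that switches on linked environment actors when its deactivation event fires.
; On CEEnviroDesactivated, it checks that ActorLink has at least one entry, then casts each to BP_MainEnvironmentInteractible and calls CEEnviroActivated on it.
; The relay is inverted: deactivating this actor activates its targets.
; BeginPlay, overlap, Tick and the construction script add no logic of their own.
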(event `self.CE_EnviroDesactivated`
  (if (`KismetArrayLibrary.Array_IsValidIndex` (`self.ActorLink`))
    (for _array_element (`self.ActorLink`)
      (bind _asbp_main_environment_interactible (cast `/Game/Blueprints/Interactible/Environments/BP_MainEnvironmentInteractible` _array_element))
      (`self.CE_EnviroActivated` _asbp_main_environment_interactible))))

(fn `UserConstructionScript`
  (`parent.UserConstructionScript`))
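; BP_RedLight is an interactible environment light whose spotlight follows activation, deactivation, light on/off and EMP events from its parent framework.
; All route into CE_TurnLight, which sets visibility and requests a switch-on sound, though the sound and noise-report logic is disconnected.
; BeginPlay derives the active state from spotlight visibility, and EMP also clears the overlap flag.
; A separate event copies this spotlight's intensity to every BP_Light in the level.
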(event `self.ReceiveBeginPlay`
  (`parent.ReceiveBeginPlay`)
  (set `self.b_isActive?` (`SceneComponent.bVisible` (`self.SpotLight`))))

(event `self.Child_Activated`
  (`self.CE_TurnLight` true :!label _label))

(event `LightOn`
  (goto _label))

(event `self.Child_Desactivated`
  (`self.CE_TurnLight` false :!label _label_2))

(event `LightOff`
  (goto _label_2))

(event `self.Child_EMP`
  (set `self.b_isOverlap` false)
  (`self.CE_TurnLight` false))

(event `CE_TurnLight`
  (params (bNewVisibility :type Boolean))
  (set `self.b_IsOn` bNewVisibility)
  (`SceneComponent.SetVisibility` (`self.SpotLight`) (`self.b_IsOn`) false)
  (if (`self.b_IsOn`)
    (`self.CE_SoundAtLamp` (`self.SoundLightOn`))))

(event `Set_all_light_intensity`
  (bind _outactors (`GameplayStatics.GetAllActorsOfClass` "/Game/Blueprints/Interactible/Environments/BP_Light.BP_Light_C"))
  (for _array_element _outactors
    (`LightComponent.SetIntensity` (`/Game/Blueprints/Interactible/Environments/BP_Light.SpotLight` _array_element) (`LightComponentBase.Intensity` (`self.SpotLight`)))))

(event `CE_SoundAtLamp`
  (params (Sound :type "SoundBase Object Reference")))

(fn `UserConstructionScript`
  (`parent.UserConstructionScript`))
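; Interactible environment door that slides its mesh along a spline when activated or deactivated, with meshes set from a data table row.
; Activation blocking-loads any assigned streaming levels, then opens, optionally gated on linked actors being on.
; Tick advances a timer into an eased spline alpha, rescaled on state change so reversals continue from the current position.
; Sounds, Niagara effects and an AI noise event accompany movement.
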(event `self.ReceiveBeginPlay`)

(event `self.ReceiveTick`
  (params (DeltaSeconds :type "Float (single-precision)"))
  (switch `/Game/Blueprints/Interactible/Environments/E_DoorState` (`self.E_DoorState`)
    (:`NewEnumerator0`
      (`self.CE_Gauge` true (`self.f_OpenDuration`)))
    (:`NewEnumerator1`
      (`self.CE_Gauge` false (`self.f_CloseDuration`)))))

(event `CE_DoorClose`
  (set `self.b_IsOn` true)
  (set `self.b_Retriggerable` true)
  (set `self.E_DoorState` "NewEnumerator4")
  (`NiagaraFunctionLibrary.SpawnSystemAtLocation` "/Game/Environments/FX/Niagara/NS_DoorClose.NS_DoorClose" (`SceneComponent.K2_GetComponentLocation` (`self.SM_LP_Big_DoorFrame`))))

(event `CE_Gauge`
  (params (b_Add :type Boolean) (f_Time :type "Float (double-precision)"))
  (if b_Add
    (if (< (`self.f_CurrentTime`) (`self.f_OpenDuration`))
      (`self.FC_SetGauge` (`GameplayStatics.GetWorldDeltaSeconds`) b_Add f_Time :!label _label)
      (`self.FC_SetDoorLocation`)
      (set `self.b_Retriggerable` false)
      (else
        (`self.CE_DoorOpen`)))
    (elif (> (`self.f_CurrentTime`) 0.0)
      (goto _label)
      (else
        (`self.CE_DoorClose`)))))

(event `CE_DoorOpen`
  (set `self.b_IsOn` false)
  (set `self.b_Retriggerable` true)
  (set `self.E_DoorState` "NewEnumerator4"))

(event `CE_OpenState`
  (if (`self.b_NeedTriggerOn`)
    (for _array_element (`self.ActorLinked`)
      (bind _b_ison (`/Game/Blueprints/Interactible/Triggers/BP_MainTriggers.b_IsOn` _array_element))
      (if (not _b_ison)
        (break)))
    (if _b_ison
      (set `self.E_DoorState` "NewEnumerator0"))
    (else
      (set `self.E_DoorState` "NewEnumerator0")
      (`self.CE_play_sound` "/Game/Audio/Sounds/Door/Big_Door_open_sound_Cue.Big_Door_open_sound_Cue")
      (`NiagaraFunctionLibrary.SpawnSystemAtLocation` "/Game/Environments/FX/Niagara/NS_DoorOpen.NS_DoorOpen" (`SceneComponent.K2_GetComponentLocation` (`self.SM_LP_Big_DoorFrame`)))
      (`self.FC_AdjustCurrentTime` :!label _label_2)
      (`AISense_Hearing.ReportNoiseEvent` (`self.K2_GetActorLocation`) 1.0 self 0.0 "Door"))))

(event `CE_CloseState`
  (set `self.E_DoorState` "NewEnumerator1")
  (`self.CE_play_sound` "/Game/Audio/Sounds/Door/Big_Door_close_sound_Cue.Big_Door_close_sound_Cue")
  (goto _label_2))

(event `self.Child_Activated`
  (if (`KismetSystemLibrary.IsValidSoftObjectReference` (`|GetArrayItem` (`self.Level`))) :!label _label_3
    (set `self.i_ArrayIndex` 0)
    (if (< (`self.i_ArrayIndex`) (`KismetArrayLibrary.Array_Length` (`self.Level`))) :!label _label_4
      (`GameplayStatics.LoadStreamLevelBySoftObjectPtr` (`|GetArrayItem` (`self.Level`) (`self.i_ArrayIndex`)) true true)
      (set `self.i_ArrayIndex` (+ (`self.i_ArrayIndex`) 1))
      (goto _label_4)
      (else
        (`self.CE_OpenState`)))
    (else
      (`self.CE_OpenState`))))

(event `self.CE_EnviroActivated`
  (goto _label_3))

(event `self.Child_Desactivated`
  (`self.CE_CloseState` :!label _label_5))

(event `self.CE_EnviroDesactivated`
  (goto _label_5))

(event `CE_play_sound`
  (params (Sound :type "SoundBase Object Reference"))
  ;[1 0.8655 0] Comment
  (`GameplayStatics.PlaySoundAtLocation` Sound (+ (`self.K2_GetActorLocation`) (0.0 0.0 100.0)) (struct) 1.0 1.0 0.0 "/Game/Audio/Sound_attenuation/SA_Door.SA_Door" null null null))

(fn `FC_AdjustCurrentTime`
  (set `self.f_CurrentTime` (`KismetMathLibrary.Lerp` 0.0 (select `/Game/Blueprints/Interactible/Environments/E_DoorState` (`self.E_DoorState`) :`NewEnumerator0` (`self.f_OpenDuration`) :`NewEnumerator1` (`self.f_CloseDuration`) :!type "Float (double-precision)") (`self.f_Alpha`))))

(fn `FC_SetDoorLocation`
  (`SceneComponent.K2_SetWorldLocation` (`self.SM_LP_Big_Door`) (`SplineComponent.GetLocationAtTime` (`self.Spline`) (`self.f_Alpha`) "World" false) false false))

(fn `FC_SetGauge`
  (params (f_DeltaSecond :type "Float (double-precision)") (b_A :type Boolean) (f_Time :type "Float (double-precision)"))
  (bind _output_get (set `self.f_CurrentTime` (+ (`self.f_CurrentTime`) (select `bool` b_A :`false` (* f_DeltaSecond -1.0) :`true` f_DeltaSecond))))
  (set `self.f_Alpha` (`|EaseFunction` (select `bool` b_A :`false` "EaseOut" :`true` "EaseIn" :!type "EEasingFunc Enum") (`KismetMathLibrary.NormalizeToRange` _output_get 0.0 f_Time) 0.0 1.0 3.5)))

(fn `UserConstructionScript`
  (bind _returnvalue (`|GetDataTableRow` "/Game/DataTables/DT_Doors.DT_Doors" (`.RowName` (break `DataTableRowHandle` (`self.DT_Doors`))))
    (:`then`
      (`|ExecutionSequence`
        (:`then_0`
          (bind (_sm_door _sm_doorframe) (break `/Game/DataTables/S_Door` _returnvalue))
          (`StaticMeshComponent.SetStaticMesh` (`self.SM_LP_Big_Door`) _sm_door))
        (:`then_1`
          (`StaticMeshComponent.SetStaticMesh` (`self.SM_LP_Big_DoorFrame`) _sm_doorframe))))))
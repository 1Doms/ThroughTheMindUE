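; BP_Pillar is an interactible environment pillar whose emissive glow switches on and off with its activation state.
; CEEnviroActivated creates a dynamic instance of the Pillar mesh's second material slot, setting a pale green emissive color and intensity.
; CEEnviroDesactivated repeats this with black and zero intensity, so each call creates a new instance.
; Nothing in this Blueprint calls either event, and its default events are disabled.
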(event `self.CE_EnviroActivated`
  (bind _pillar (`self.Pillar`))
  (bind _returnvalue (`PrimitiveComponent.CreateDynamicMaterialInstance` _pillar 1 (`PrimitiveComponent.GetMaterial` _pillar 1) "None"))
  (set `self.Mat` _returnvalue)
  (`MaterialInstanceDynamic.SetScalarParameterValue` (`self.Mat`) "Emissive Intensity" 3.0)
  (`MaterialInstanceDynamic.SetVectorParameterValue` (`self.Mat`) "Emissive_Color" (struct :`R` 0.784314 :`G` 1.0 :`B` 0.615686 :`A` 1.0))
  (`PrimitiveComponent.SetMaterial` (`self.Pillar`) 1 (`self.Mat`)))

(event `self.CE_EnviroDesactivated`
  (bind _pillar (`self.Pillar`))
  (bind _returnvalue (`PrimitiveComponent.CreateDynamicMaterialInstance` _pillar 1 (`PrimitiveComponent.GetMaterial` _pillar 1) "None"))
  (set `self.Mat` _returnvalue)
  (`MaterialInstanceDynamic.SetScalarParameterValue` (`self.Mat`) "Emissive Intensity" 0.0)
  (`MaterialInstanceDynamic.SetVectorParameterValue` (`self.Mat`) "Emissive_Color" (struct :`A` 1.0))
  (`PrimitiveComponent.SetMaterial` (`self.Pillar`) 1 (`self.Mat`)))

(fn `UserConstructionScript`
  (`parent.UserConstructionScript`))
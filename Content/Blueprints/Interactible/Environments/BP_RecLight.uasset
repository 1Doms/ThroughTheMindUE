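; BP_RecLight is an interactible environment rect light that turns on and off through parent activation hooks or LightOn/LightOff events.
; Both paths feed one event that sets the light's visibility and, when on, plays a sound at the lamp and reports a "Light"-tagged noise event.
; An EMP clears the overlap flag and switches it off.
; A separate event copies its intensity to every BP_Light spotlight in the level.
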(event `self.ReceiveBeginPlay`
  (`parent.ReceiveBeginPlay`))

(event `self.Child_Activated`
  (`self.CE_TurnLight` true :!label _label))

(event `LightOn`
  (goto _label))

(event `self.Child_Desactivated`
  (`self.CE_TurnLight` false :!label _label_2))

(event `LightOff`
  (goto _label_2))

(event `self.Child_EMP`
  (set `self.b_isOverlap` false)
  (`self.CE_TurnLight` false))

(event `CE_TurnLight`
  (params (bNewVisibility :type Boolean))
  (set `self.b_IsOn` bNewVisibility)
  (`SceneComponent.SetVisibility` (`self.RectLight`) (`self.b_IsOn`) false)
  (if (`self.b_IsOn`)
    (`self.CE_SoundAtLamp` (`self.SoundLightOn`))))

(event `Set_all_light_intensity`
  (bind _outactors (`GameplayStatics.GetAllActorsOfClass` "/Game/Blueprints/Interactible/Environments/BP_Light.BP_Light_C"))
  (for _array_element _outactors
    (`LightComponent.SetIntensity` (`/Game/Blueprints/Interactible/Environments/BP_Light.SpotLight` _array_element) (`LightComponentBase.Intensity` (`self.RectLight`)))))

(event `CE_SoundAtLamp`
  (params (Sound :type "SoundBase Object Reference"))
  (`GameplayStatics.PlaySoundAtLocation` Sound (`SceneComponent.K2_GetComponentLocation` (`self.Lamp`)) (struct) 0.25 1.0 0.0 "/Game/Audio/Sound_attenuation/SA_Long.SA_Long" null null null)
  (`AISense_Hearing.ReportNoiseEvent` (`SceneComponent.K2_GetComponentLocation` (`self.Lamp`)) 1.0 null 0.0 "Light"))

(fn `UserConstructionScript`
  (`parent.UserConstructionScript`))
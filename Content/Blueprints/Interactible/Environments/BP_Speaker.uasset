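; BP_Speaker is an environment speaker that plays dialogue announcements and controls the alarm siren.
; CE_sound_at_location plays two spatialized alarm sounds with short delays before the requested dialogue at the speaker's location.
; Two special DialogueName values instead switch the siren on or off through its volume multiplier.
; The siren toggle also activates or deactivates every BP_RedLight, gathered once at BeginPlay.
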(event `self.ReceiveBeginPlay`
  (`parent.ReceiveBeginPlay`)
  (bind _outactors (`GameplayStatics.GetAllActorsOfClass` "/Game/Blueprints/Interactible/Environments/BP_RedLight.BP_RedLight_C"))
  (set `self.RedLights` _outactors))

(event `self.Child_Activated`)

(event `CE_sound_at_location`
  (params (`Dialogue name` :type "/Game/Dialogues/EDialoguesNames Enum" :default "NewEnumerator0") (AttenuationSettings :type "SoundAttenuation Object Reference"))
  (bind _returnvalue (`self.K2_GetActorLocation`))
  (if (`|EnumEquality` `Dialogue name` "NewEnumerator3")
    (`self.CE_Siren_On`)
    (elif (`|EnumEquality` `Dialogue name` "NewEnumerator4")
      (`self.CE_Siren_Off`)
      (else
        (`GameplayStatics.PlaySoundAtLocation` "/Game/Audio/Sounds/Enviro/Speakers/Alarm_3_sound_Cue.Alarm_3_sound_Cue" _returnvalue (struct) 1.0 1.0 0.0 "/Game/Audio/Sound_attenuation/SA_Speakers.SA_Speakers" null null null)
        (`KismetSystemLibrary.Delay` 1.0)
        (`GameplayStatics.PlaySoundAtLocation` "/Game/Audio/Sounds/Enviro/Speakers/Alarm_3_sound_Cue.Alarm_3_sound_Cue" _returnvalue (struct) 1.0 1.0 0.0 "/Game/Audio/Sound_attenuation/SA_Speakers.SA_Speakers" null null null)
        (`KismetSystemLibrary.Delay` 1.5)
        (`/Game/Blueprints/BFL_TTM.Play_Dialogue` `Dialogue name` _returnvalue AttenuationSettings)))))

(event `CE_Siren_On`
  (`AudioComponent.SetVolumeMultiplier` (`self.Siren_sound_Cue`) 1.0)
  (for _array_element (`self.RedLights`)
    (`self.Child_Activated` _array_element)))

(event `CE_Siren_Off`
  (`AudioComponent.SetVolumeMultiplier` (`self.Siren_sound_Cue`) 0.0)
  (for _array_element (`self.RedLights`)
    (`self.Child_Desactivated` _array_element)))

(fn `UserConstructionScript`
  (`parent.UserConstructionScript`))
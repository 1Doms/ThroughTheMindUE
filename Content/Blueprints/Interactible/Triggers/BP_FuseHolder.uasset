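; Fuse holder trigger where the player inserts a carried BP_Fuse and holds input to push it home, activating linked actors once it rotates locked.
; A Tick-driven state machine fills or drains a gauge that moves the socket, drives push audio and reports noise.
; Released pushes auto-retract after a delay; cancelling unlocks or pulls the fuse, deactivating links and dropping it when empty.
; Interaction freezes movement and clamps the camera around the holder.
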(event `self.ReceiveBeginPlay`
  (bind _fuseholder (`self.FuseHolder`))
  (`self.CE_spawn_sound_push`)
  (if (and (`self.b_StartWithFuse?`) (not (`self.FC_FuseHasChild`)))
    (bind _returnvalue (`|SpawnActorFromClass` "/Game/Blueprints/Interactible/Items/BP_Fuse.BP_Fuse_C" (`KismetMathLibrary.MakeTransform` (0.0 0.0 0.0)) "AlwaysSpawn" "OverrideRootScale" null null))
    (set `self.As BP Fuse` _returnvalue)
    (`self.CE_AddFuse`)
    (if (`SceneComponent.DoesSocketExist` _fuseholder "SocketGrip")
      (set `self.SocketGrip` (`SceneComponent.GetSocketTransform` _fuseholder "SocketGrip" "RTS_World")))
    (else
      (set `self.InteractionFeedbackText` (`self.FeedbackEmpty`)))))

(event `CE_Init`
  (bind _asbp_player_character (cast `/Game/Blueprints/Characters/BP_PlayerCharacter` (`GameplayStatics.GetPlayerCharacter` 0)))
  (set `self.Player_Ref` _asbp_player_character)
  (set `self.Physics Handle` (`/Game/Blueprints/Characters/BP_PlayerCharacter.PhysicsHandle` (`self.Player_Ref`)))
  (`/Engine/EditorBlueprintResources/StandardMacros.DoOnce` false
    (:`Completed`
      (`SceneComponent.K2_SetRelativeRotation` (`self.FuseSocket`) (`self.FC_GetSocketRot`) false false))))

(event `CE_DisablePlayerMovement`
  (`CharacterMovementComponent.DisableMovement` (`Character.CharacterMovement` (`self.Player_Ref`)))
  (set `/Game/Blueprints/Characters/BP_PlayerCharacter.ObjectInteractionRef` self (`self.Player_Ref`))
  (`self.CE_FocusCam` true))

(event `self.ReceiveTick`
  (params (DeltaSeconds :type "Float (single-precision)"))
  (bind _alpha (`self.Alpha`))
  (switch `/Game/Blueprints/Interactible/Triggers/E_FuseState` (`self.E_FuseState`)
    (:`NewEnumerator0`
      (`self.CE_SoundPushing` 0.0 :!label _label))
    (:`NewEnumerator1`
      (`self.CE_Gauge` true (`self.f_PushDuration`))
      ;[1 0.7634 0] Comment
      (`self.CE_SoundPushing` (`self.Max volume push`) :!label _label_2)
      (`AISense_Hearing.ReportNoiseEvent` (`self.K2_GetActorLocation`) 1.0 self 0.0 "Fuse")
      (`MeshComponent.SetScalarParameterValueOnMaterials` (`self.Jauge`) "Alpha" _alpha)
      (`MeshComponent.SetScalarParameterValueOnMaterials` (`self.RadialJauge`) "Alpha" _alpha)
      (`self.CE_RightInteraction` (`self.As BP Fuse`)))
    (:`NewEnumerator2`
      (`self.CE_Gauge` false (`self.f_AutoPullDuration`))
      (goto _label_2))
    (:`NewEnumerator3`
      (`self.CE_Gauge` false (`self.f_PullDuration`))
      (goto _label_2))
    (:`NewEnumerator5`
      (goto _label))))

(event `CE_RotationAnim`
  (bind _returnvalue (`self.FC_GetSocketRot`))
  (bind _returnvalue_2 (`self.FC_GetSocketRot`))
  (`|ExecutionSequence`
    (:`then_0`
      (goto _label_6 :!via `Reset`))
    (:`then_1`
      (`/Engine/EditorBlueprintResources/StandardMacros.DoOnce` false :!label _label_3
        (:`Completed`
          (`|ExecutionSequence`
            (:`then_0`
              (bind (_direction _alpha) (`Timeline|Timeline` :!via `Stop` :!label _label_4)
                (:`Update`
                  (`SceneComponent.K2_SetRelativeRotation` (`self.FuseSocket`) (`|EaseFunction` "ExpoInOut" _alpha (`KismetMathLibrary.MakeRotator` (+ (.roll _returnvalue) 90.0) (.pitch _returnvalue) (.yaw _returnvalue)) _returnvalue) false false)
                  (`self.CE_DisablePlayerMovement`)
                  (`self.CE_RightInteraction` (`self.As BP Fuse`)))
                (:`Finished`
                  (`self.CE_DelockRotFinished`)
                  (`self.CE_SmokeEject`))))
            (:`then_1`
              (bind (_direction_2 _alpha_2) (`Timeline|RotationTimeline` :!via `PlayFromStart` :!label _label_5)
                (:`Update`
                  (`SceneComponent.K2_SetRelativeRotation` (`self.FuseSocket`) (`|EaseFunction` "ExpoInOut" _alpha_2 _returnvalue_2 (`KismetMathLibrary.MakeRotator` (+ (.roll _returnvalue_2) 90.0) (.pitch _returnvalue_2) (.yaw _returnvalue_2))) false false)
                  (set `self.E_FuseState` "NewEnumerator0")
                  (`self.CE_RightInteraction` (`self.As BP Fuse`)))
                (:`Finished`
                  (`self.CE_LockRotFinished`))))))))))

(event `CE_LockRotFinished`
  (`self.CE_Activate`)
  (set `self.InteractionFeedbackText` (`self.FeedbackLock`))
  (`self.CE_RightInteraction` null))

(event `CE_FocusCam`
  (params (`b_IsFocus?` :type Boolean))
  (set `self.B Is Focus?` `b_IsFocus?`)
  (`|ExecutionSequence`
    (:`then_0`
      (set `PlayerCameraManager.ViewPitchMin` (select `bool` (`self.B Is Focus?`) :`false` -90.0 :`true` (`KismetMathLibrary.FClamp` (- (`self.FC_GetCameraRot`) (`self.f_FocusAngle`)) -75.0 90.0) :!type "Float (single-precision)") (`GameplayStatics.GetPlayerCameraManager` 0)))
    (:`then_1`
      (set `PlayerCameraManager.ViewPitchMax` (select `bool` (`self.B Is Focus?`) :`false` 90.0 :`true` (+ (`self.FC_GetCameraRot`) (`self.f_FocusAngle`)) :!type "Float (single-precision)") (`GameplayStatics.GetPlayerCameraManager` 0)))
    (:`then_2`
      (set `PlayerCameraManager.ViewYawMin` (select `bool` (`self.B Is Focus?`) :`true` (- (`.ReturnValue_Yaw` (`self.FC_GetCameraRot`)) (`self.f_FocusAngle`)) :!type "Float (single-precision)") (`GameplayStatics.GetPlayerCameraManager` 0)))
    (:`then_3`
      (set `PlayerCameraManager.ViewYawMax` (select `bool` (`self.B Is Focus?`) :`false` 359.0 :`true` (+ (`.ReturnValue_Yaw` (`self.FC_GetCameraRot`)) (`self.f_FocusAngle`))) (`GameplayStatics.GetPlayerCameraManager` 0)))))

(event `CE_ReverseRotation`
  (`|ExecutionSequence`
    (:`then_0`
      (goto _label_3 :!via `Reset`))
    (:`then_1`
      (`/Engine/EditorBlueprintResources/StandardMacros.DoOnce` false :!label _label_6
        (:`Completed`
          (`|ExecutionSequence`
            (:`then_0`
              (goto _label_5 :!via `Stop`))
            (:`then_1`
              (`self.CE_SoundAtFuse` "/Game/Audio/Sounds/Fuse/Fuse_out_sound_Cue.Fuse_out_sound_Cue")
              (goto _label_4 :!via `PlayFromStart`))))))))

(event `CE_DelockRotFinished`
  (`self.CE_PullFuse`)
  (`self.CE_Desactivate`))

(event `CE_Gauge`
  (params (`b_Add?` :type Boolean) (f_TimeRange :type "Float (double-precision)"))
  (if `b_Add?`
    (if (< (`self.f_CurrentTime`) (`self.f_PushDuration`))
      (`self.FC_SetGauge` (`GameplayStatics.GetWorldDeltaSeconds`) `b_Add?` f_TimeRange :!label _label_7)
      (`self.FC_SetFuseLocation`)
      (else
        (`self.CE_GaugeFull`)))
    (elif (> (`self.f_CurrentTime`) 0.0)
      (goto _label_7)
      (else
        (`self.CE_GaugeEmpty`)))))

(event `CE_EnablePlayerMovement`
  (`CharacterMovementComponent.SetMovementMode` (`Character.CharacterMovement` (`self.Player_Ref`)) "MOVE_Walking" 0)
  (set `/Game/Blueprints/Characters/BP_PlayerCharacter.ObjectInteractionRef` null (`self.Player_Ref`))
  (`self.CE_FocusCam` false))

(event `CE_SmokeEject`
  (`NiagaraFunctionLibrary.SpawnSystemAtLocation` "/Game/Environments/FX/Niagara/NS_FuzeEjection.NS_FuzeEjection" (`SceneComponent.K2_GetComponentLocation` (`self.InLocation`)) (`self.FC_GetSocketRot`)))

(event `CE_GaugeFull`
  (`self.CE_RotationAnim`)
  (`self.CE_SoundAtFuse` "/Game/Audio/Sounds/Fuse/Fuse_in_sound_Cue.Fuse_in_sound_Cue"))

(event `CE_RightInteraction`
  (params (`Right Arm Interact` :type "/Game/Blueprints/Interactible/BP_MainInteractible Object Reference"))
  (bind _player_ref (`self.Player_Ref`))
  (if (< (`KismetMathLibrary.Vector_Distance` (`self.K2_GetActorLocation` _player_ref) (`self.K2_GetActorLocation`)) 128.0)
    (bind _asabp_player (cast `/Game/Blueprints/Characters/Animations/Blueprints/ABP_Player` (`SkeletalMeshComponent.GetAnimInstance` (`/Game/Blueprints/Characters/BP_PlayerCharacter.FirstPersonMesh` _player_ref))))
    (`/Game/Blueprints/Characters/Animations/Blueprints/ABP_Player.CE_RightArm` _asabp_player `Right Arm Interact`)))

(event `CE_GaugeEmpty`
  (`self.CE_RemoveFuse`)
  (set `self.E_FuseState` "NewEnumerator5"))

(event `CE_RemoveFuse`
  (bind _returnvalue (`SceneComponent.GetChildComponent` (`self.FuseSocket`) 0))
  (`/Engine/EditorBlueprintResources/StandardMacros.IsValid` _returnvalue
    (:`Is Valid`
      (`SceneComponent.K2_DetachFromComponent` _returnvalue "KeepWorld" "KeepWorld" "KeepWorld" true)
      (`self.CE_NothingGateClose`)
      (`/Game/Blueprints/Interactible/Items/BP_MainItem.CE_DropItem` (`self.As BP Fuse`))
      (`self.CE_EnablePlayerMovement`)
      (set `self.As BP Fuse` null)
      (bind _returnvalue_2 (`KismetSystemLibrary.K2_SetTimerDelegate` (delegate `CE_OutOfRange`) 0.5 true))
      (set `self.TH_OutOfRange` _returnvalue_2)
      (set `self.InteractionFeedbackText` (`self.FeedbackRemove`)))))

(event `CE_OutOfRange`
  (if (< (`self.GetDistanceTo` (`GameplayStatics.GetPlayerCharacter` 0)) (`self.f_OutOfRange`))
    (set `self.b_IsInteractible?` false)
    (`MeshComponent.SetScalarParameterValueOnMaterials` (`self.Jauge`) "Alpha" 0.5)
    (`KismetSystemLibrary.Delay` 0.25)
    (`MeshComponent.SetScalarParameterValueOnMaterials` (`self.Jauge`) "Alpha" 0.0)
    (else
      (`self.CE_NothingGateOpen`)
      (set `self.b_IsInteractible?` true)
      (`KismetSystemLibrary.K2_ClearAndInvalidateTimerHandle` (`self.TH_OutOfRange`)))))

(event `CE_AddFuse`
  (bind _returnvalue (`PhysicsHandleComponent.GetGrabbedComponent` (`self.Physics Handle`)))
  (`self.CE_Init`)
  (`self.As BP Fuse`
    (:`then`
      _)
    (:`else`
      (`/Engine/EditorBlueprintResources/StandardMacros.IsValid` _returnvalue
        (:`Is Valid`
          (set `self.GrabItemRef` (`ActorComponent.GetOwner` _returnvalue))
          (bind _asbp_fuse (cast `/Game/Blueprints/Interactible/Items/BP_Fuse` (`self.GrabItemRef`)))
          (set `self.As BP Fuse` _asbp_fuse)))))
  (`/Game/Blueprints/Interactible/Items/BP_Fuse.CE_PutToHolder` (`self.As BP Fuse`))
  (`SceneComponent.K2_AttachToComponent` (`/Game/Blueprints/Interactible/Items/BP_MainItem.StaticMesh` (`self.As BP Fuse`)) (`self.FuseSocket`) "None" "SnapToTarget" "SnapToTarget" "KeepWorld" true)
  (set `self.E_FuseState` "NewEnumerator1")
  (set `self.InteractionFeedbackText` (`self.FeedbackFuze`)))

(event `/Game/Blueprints/Interactible/BPI_Interaction.Interaction`
  (params (InputState :type "/Game/Blueprints/Characters/E_InputState Enum" :default "NewEnumerator0") (PlayerRef :type "/Game/Blueprints/Characters/BP_PlayerCharacter Object Reference") (Item :type "/Game/Blueprints/Interactible/BP_MainInteractible Object Reference"))
  (set `self.Input State` InputState)
  (`self.CE_Init`)
  (if (not (and (`KismetSystemLibrary.IsValid` (`PhysicsHandleComponent.GetGrabbedComponent` (`self.Physics Handle`))) (`self.FC_FuseHasChild`)))
    (switch `/Game/Blueprints/Characters/E_InputState` (`self.Input State`)
      (:`NewEnumerator0`
        (switch `/Game/Blueprints/Interactible/Triggers/E_FuseState` (`self.E_FuseState`)
          (:`NewEnumerator0`
            (`/Engine/EditorBlueprintResources/StandardMacros.Gate` false :!label _label_8
              (:`Exit`
                (`self.CE_InputCanceled`))))
          (:`NewEnumerator1`
            (`self.CE_InputPushing` :!label _label_9)
            (`self.CE_LockGateClose`))
          (:`NewEnumerator4`
            (goto _label_9))
          (:`NewEnumerator2`
            (goto _label_9))
          (:`NewEnumerator5`
            (`/Engine/EditorBlueprintResources/StandardMacros.Gate` false :!label _label_10
              (:`Exit`
                (goto _label_9))))))
      (:`NewEnumerator3`
        (`self.CE_InputCanceled`))
      (:`NewEnumerator4`
        (`self.CE_InputCompleted`)))))

(event `CE_LockGateOpen`
  (goto _label_8 :!via `Open`))

(event `CE_LockGateClose`
  (goto _label_8 :!via `Close`))

(event `CE_NothingGateOpen`
  (goto _label_10 :!via `Open`))

(event `CE_NothingGateClose`
  (goto _label_10 :!via `Close`))

(event `CE_PullFuse`
  (set `self.E_FuseState` "NewEnumerator3")
  (`self.CE_DisablePlayerMovement`)
  ;[1 1 1] Smoke out sound WHERE?
  (`self.PUllingSound` null)
  (`self.FC_AdjustCurrentTime`))

(event `CE_InputPushing`
  (if (not (`self.FC_FuseHasChild`))
    (`self.CE_AddFuse`)
    (elif (`|EnumInequality` (`self.E_FuseState`) "NewEnumerator0")
      (`|ExecutionSequence`
        (:`then_0`
          (set `self.E_FuseState` "NewEnumerator1")
          (`self.CE_DisablePlayerMovement`)
          (`self.FC_AdjustCurrentTime` :!label _label_11))
        (:`then_1`
          (`KismetSystemLibrary.RetriggerableDelay` (`self.f_WaitingDuration`))
          (if (`|EnumEquality` (`self.E_FuseState`) "NewEnumerator4")
            (set `self.E_FuseState` "NewEnumerator2")
            (goto _label_11)))))))

(event `CE_InputCanceled`
  (if (`self.FC_FuseHasChild`)
    (switch `/Game/Blueprints/Interactible/Triggers/E_FuseState` (`self.E_FuseState`)
      (:`NewEnumerator0`
        (`self.CE_ReverseRotation`))
      (:`NewEnumerator1`
        (`self.CE_PullFuse` :!label _label_12))
      (:`NewEnumerator4`
        (goto _label_12))
      (:`NewEnumerator2`
        (goto _label_12))
      (:`NewEnumerator5`
        (goto _label_12)))))

(event `CE_InputCompleted`
  (switch `/Game/Blueprints/Interactible/Triggers/E_FuseState` (`self.E_FuseState`)
    (:`NewEnumerator0`
      (`self.CE_LockGateOpen`))
    (:`NewEnumerator1`
      (set `self.E_FuseState` "NewEnumerator4")))
  (`self.CE_EnablePlayerMovement`))

(event `CE_Activate`
  (set `self.b_IsOn` true)
  (`self.CE_ForEachActorLink` true))

(event `CE_Desactivate`
  (set `self.b_IsOn` false)
  (`self.CE_ForEachActorLink` false))

(event `CE_SoundAtFuse`
  (params (Sound :type "SoundBase Object Reference"))
  ;[1 0.8524 0.1277] Comment
  (`GameplayStatics.PlaySoundAtLocation` Sound (`SceneComponent.K2_GetComponentLocation` (`self.FuseSocket`)) (struct) 1.0 1.0 0.0 "/Game/Audio/Sound_attenuation/SA_Generic.SA_Generic" null null null))

(event `PullingSound`
  (params (Sound :type "SoundBase Object Reference"))
  (`GameplayStatics.PlaySoundAtLocation` Sound (`SceneComponent.K2_GetComponentLocation` (`self.FuseSocket`)) (struct) 1.0 1.0 0.0 "/Game/Audio/Sound_attenuation/SA_Generic.SA_Generic" null null null))

(event `CE_spawn_sound_push`
  ;[1 0.7634 0] Comment
  (bind _returnvalue (`GameplayStatics.SpawnSoundAttached` "/Game/Audio/Sounds/Fuse/Fuse_push_sound_Cue.Fuse_push_sound_Cue" (`self.FuseHolder`) "None" (0.0 0.0 0.0) (struct) "SnapToTarget" false 1.0 1.0 0.0 "/Game/Audio/Sound_attenuation/SA_Generic.SA_Generic" null false))
  (bind _output_get (set `self.Push_sound_ref` _returnvalue))
  (`AudioComponent.SetVolumeMultiplier` _output_get (`self.Max volume push`))
  (`GameplayStatics.SetSoundMixClassOverride` "/Game/Audio/Sounds_mix/SCM_TTM.SCM_TTM" "/Game/Audio/Sounds_class/SC_FusePush.SC_FusePush" 0.5 1.0 0.0)
  (`GameplayStatics.PushSoundMixModifier` "/Game/Audio/Sounds_mix/SCM_TTM.SCM_TTM"))

(event `CE_SoundPushing`
  (params (NewVolumeMultiplier :type "Float (single-precision)"))
  (`AudioComponent.SetVolumeMultiplier` (`self.Push_sound_ref`) NewVolumeMultiplier)
  (`AudioComponent.SetPitchMultiplier` (`self.Push_sound_ref`) (`self.FC_AlphaOnePlus`)))

(event `CE_ResetSoundPushing`
  (`/Engine/EditorBlueprintResources/StandardMacros.DoOnce` false :!via `Reset`))

(event `CE_PlaySoundAtGauge`
  (`GameplayStatics.PlaySoundAtLocation` "/Game/Audio/Sounds/Fuse/Bip.Bip" (`SceneComponent.K2_GetComponentLocation` (`self.Jauge`)) (struct) 1.0 1.0 0.0 "/Game/Audio/Sound_attenuation/SA_Generic.SA_Generic" null null null)
  (`MeshComponent.SetScalarParameterValueOnMaterials` (`self.Jauge`) "Alpha" 0.5)
  (`KismetSystemLibrary.Delay` 0.1)
  (`MeshComponent.SetScalarParameterValueOnMaterials` (`self.Jauge`) "Alpha" 0.0))

(fn `FC_AdjustCurrentTime`
  (set `self.f_CurrentTime` (`KismetMathLibrary.Lerp` 0.0 (select `/Game/Blueprints/Interactible/Triggers/E_FuseState` (`self.E_FuseState`) :`NewEnumerator1` (`self.f_PushDuration`) :`NewEnumerator2` (`self.f_AutoPullDuration`) :`NewEnumerator3` (`self.f_PullDuration`)) (`self.Alpha`))))

(fn `FC_AlphaOnePlus`
  (returns (ReturnValue :type "Float (double-precision)"))
  (return (+ (`self.Alpha`) 1.0)))

(fn `FC_FuseHasChild`
  (returns (b_hasChild :type Boolean))
  (return (`KismetSystemLibrary.IsValid` (`SceneComponent.GetChildComponent` (`self.FuseSocket`) 0))))

(fn `FC_GetCameraRot`
  (returns (ReturnValue_Pitch :type "Float (single-precision)") (ReturnValue_Yaw :type "Float (single-precision)"))
  (bind (_returnvalue_roll _returnvalue_pitch _returnvalue_yaw) (`KismetMathLibrary.BreakRotator` (`KismetMathLibrary.FindLookAtRotation` (`SceneComponent.K2_GetComponentLocation` (`/Game/Blueprints/Characters/BP_PlayerCharacter.FirstPersonCamera` (`self.Player_Ref`))) (`SceneComponent.K2_GetComponentLocation` (`self.Box`)))))
  (return _returnvalue_pitch _returnvalue_yaw))

(fn `FC_GetSocketRot`
  (returns (ReturnValue :type "Rotator Structure"))
  (return (`KismetMathLibrary.FindLookAtRotation` (`SceneComponent.RelativeLocation` (`self.InLocation`)) (`SceneComponent.RelativeLocation` (`self.OutLocation`)))))

(fn `FC_SetFuseLocation`
  (`SceneComponent.K2_SetWorldLocation` (`self.FuseSocket`) (`KismetMathLibrary.VLerp` (`SceneComponent.K2_GetComponentLocation` (`self.OutLocation`)) (`SceneComponent.K2_GetComponentLocation` (`self.InLocation`)) (`|EaseFunction` "EaseOut" (`self.Alpha`) 0.0 1.0 1.5)) false false))

(fn `FC_SetGauge`
  (params (f_DeltaSecond :type "Float (double-precision)") (`b_Add?` :type Boolean) (f_TimeRange :type "Float (double-precision)"))
  (set `self.f_CurrentTime` (+ (`self.f_CurrentTime`) (select `bool` `b_Add?` :`false` (* f_DeltaSecond -1.0) :`true` f_DeltaSecond)))
  (set `self.Alpha` (`KismetMathLibrary.NormalizeToRange` (`self.f_CurrentTime`) 0.0 f_TimeRange)))

(fn `UserConstructionScript`)
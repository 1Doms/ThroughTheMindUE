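; BP_Radio is an interactible radio that toggles its audio on and off and makes impact sounds when knocked around.
; Interaction input runs a FlipFlop behind a DoOnce that resets on release, pausing or resuming audio and swapping the screen material.
; The Desactived event jumps straight to the off branch without changing the FlipFlop state.
; Component hits play an impact cue at the hit location when the radio moves fast enough.
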(event `/Game/Blueprints/Interactible/BPI_Interaction.Desactived`
  (`AudioComponent.SetPaused` (`self.Audio`) true :!label _label)
  (`PrimitiveComponent.SetMaterial` (`self.Radio`) 1 "/Game/Environments/Props/Materials/Instances/MI_Black.MI_Black"))

(event `/Game/Blueprints/Interactible/BPI_Interaction.Interaction`
  (params (InputState :type "/Game/Blueprints/Characters/E_InputState Enum" :default "NewEnumerator0") (PlayerRef :type "/Game/Blueprints/Characters/BP_PlayerCharacter Object Reference") (Item :type "/Game/Blueprints/Interactible/BP_MainInteractible Object Reference"))
  (switch `/Game/Blueprints/Characters/E_InputState` InputState
    (:`NewEnumerator2`
      (`/Engine/EditorBlueprintResources/StandardMacros.DoOnce` false :!label _label_2
        (:`Completed`
          (`/Engine/EditorBlueprintResources/StandardMacros.FlipFlop`
            (:`A`
              (goto _label))
            (:`B`
              (`AudioComponent.SetPaused` (`self.Audio`) false)
              (`PrimitiveComponent.SetMaterial` (`self.Radio`) 1 "/Game/Environments/Props/Materials/Instances/MI_RadioScreen.MI_RadioScreen"))))))
    (:`NewEnumerator3`
      (goto _label_2 :!via `Reset`))
    (:`NewEnumerator4`
      (goto _label_2 :!via `Reset`))))

(event `self.Radio.OnComponentHit`
  (params (HitComponent :type "PrimitiveComponent Object Reference") (OtherActor :type "Actor Object Reference") (OtherComp :type "PrimitiveComponent Object Reference") (NormalImpulse :type "Vector Structure") (Hit :type "HitResult Structure (by ref)"))
  (if (> (`KismetMathLibrary.VSize` (`SceneComponent.GetComponentVelocity` (`self.Radio`))) 150.0)
    (`GameplayStatics.PlaySoundAtLocation` "/Game/Audio/Sounds/Enviro/Radio/RadioImpact_Cue.RadioImpact_Cue" (`.Location` (`GameplayStatics.BreakHitResult` Hit)) (struct) 1.0 1.0 0.0 "/Game/Audio/Sound_attenuation/SA_Mid.SA_Mid" null null null)))

(fn `UserConstructionScript`
  (`parent.UserConstructionScript`))
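; Security camera trigger meant to detect characters, switch linked actors and report noise to AI.
; On BeginPlay it sizes the decal and aims the mesh at the trigger box; on/off events only set the state.
; Box-trace detection with static and spline-patrol/chase states, line-of-sight checks and delayed reset is present but disconnected, as Tick only casts the player.
; Detection events swap decal materials and play sounds; construction draws a debug box.
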(event `CameraOn`
  (set `self.E_State` "NewEnumerator0" :!label _label))

(event `/Game/Blueprints/Interactible/BPI_Interaction.Activated`
  (goto _label))

(event `/Game/Blueprints/Interactible/BPI_Interaction.Desactived`
  (set `self.E_State` "NewEnumerator5" :!label _label_2))

(event `CameraOff`
  (goto _label_2))

(event `self.ReceiveBeginPlay`
  (set `self.v3_TargetLocation` (`SceneComponent.K2_GetComponentLocation` (`self.Box`)))
  (set `self.v3_CurrentLocation` (`self.v3_TargetLocation`))
  (`SceneComponent.SetRelativeScale3D` (`self.Decal`) (* (1.0 1.0 1.0) (/ (`self.f_BoxSize`) 100.0)))
  (`self.FC_CameraLookAtOverlap`))

(event `self.ReceiveTick`
  (params (DeltaSeconds :type "Float (single-precision)"))
  (cast `/Game/Blueprints/Characters/BP_PlayerCharacter` (`GameplayStatics.GetPlayerCharacter` 0)))

(event `CE_ActorDetected`
  (set `self.b_IsDetected` true)
  (`self.CE_ForEachActorLink` true)
  (`DecalComponent.SetDecalMaterial` (`self.Decal`) "/Game/Environments/Decals/M_detector_Inst.M_detector_Inst")
  (`self.CE_SoundAtCamera` (`self.ActorDetected`)))

(event `CE_ResetTime`
  (`KismetSystemLibrary.RetriggerableDelay` (`self.f_ResetTime`))
  (set `self.b_IsDetected` false)
  (`/Engine/EditorBlueprintResources/StandardMacros.DoOnce` false :!label _label_3
    (:`Completed`
      (`self.CE_NothingDetected`))))

(event `CE_RefreshResetTime`
  (goto _label_3 :!via `Reset`))

(event `CE_OnOverLap`
  ;[0.9497 1 0] SOUND
  (`self.CE_SoundAtCamera` (`self.OnOverlapSound`)))

(event `CE_NothingDetected`
  ;[1 1 1] Comment
  (`self.CE_ForEachActorLink` false)
  (`DecalComponent.SetDecalMaterial` (`self.Decal`) "/Game/Environments/Decals/M_detector_Inst1.M_detector_Inst1")
  ;[1 0.9814 0] SOUND
  (`self.CE_SoundAtCamera` (`self.DetectedNothing`)))

(event `CE_SoundAtCamera`
  (params (Sound :type "SoundBase Object Reference"))
  ;[1 0.9954 0] SoundAtCamera
  (`GameplayStatics.PlaySoundAtLocation` Sound (`SceneComponent.K2_GetComponentLocation` (`self.CameraMesh`)) (struct) 0.3 1.0 0.0 "/Game/Audio/Sound_attenuation/SA_Generic.SA_Generic" null null null)
  (`AISense_Hearing.ReportNoiseEvent` (`SceneComponent.K2_GetComponentLocation` (`self.Box`)) 1.0 self 0.0 "MovementDetector"))

(event `Refres_debug_box`
  (`KismetSystemLibrary.DrawDebugBox` (`self.K2_GetActorLocation`) (`KismetMathLibrary.Conv_DoubleToVector` (`self.f_BoxSize`)) (struct :`R` 1.0 :`B` 0.068793 :`A` 1.0) (struct) 1.0 10.0))

(fn `FC_CameraLookAtOverlap`
  (bind _cameramesh (`self.CameraMesh`))
  (bind _returnvalue (`KismetMathLibrary.FindLookAtRotation` (`SceneComponent.K2_GetComponentLocation` _cameramesh) (`self.v3_CurrentLocation`)))
  (`SceneComponent.K2_SetWorldRotation` _cameramesh _returnvalue false false)
  (`SceneComponent.K2_SetWorldLocationAndRotation` (`self.Decal`) (`self.v3_CurrentLocation`) _returnvalue false false))

(fn `FC_Get3`
  (params (Distance :type "Float (double-precision)"))
  (returns (Size :type "Float (double-precision)") (Lenght :type "Float (double-precision)"))
  (bind _returnvalue (/ Distance 100.0))
  (bind _f_boxsize (`self.f_BoxSize`))
  (return (/ (/ _f_boxsize 1.5) _returnvalue) (/ _f_boxsize _returnvalue)))

(fn `FC_GetSplineLocation`
  (returns (Output_Get :type "Vector Structure"))
  (bind _f_timetospline (`self.f_TimeToSpline`))
  (if (>= (`self.f_SplineCurrentTime`) _f_timetospline)
    (set `self.f_SplineCurrentTime` 0.0)
    (else
      (bind _output_get (set `self.f_SplineCurrentTime` (+ (`GameplayStatics.GetWorldDeltaSeconds`) (`self.f_SplineCurrentTime`))))
      (bind _output_get_2 (set `self.v3_TargetLocation` (`SplineComponent.GetLocationAtTime` (`self.TrigerBoxPath`) (`KismetMathLibrary.NormalizeToRange` _output_get 0.0 _f_timetospline) "World" false)))
      (return _output_get_2))))

(fn `FC_IsCharacterVisible`
  (returns (OutHit :type "HitResult Structure") (IsVisible :type Boolean))
  (bind (_outhit _returnvalue) (`KismetSystemLibrary.LineTraceSingle` (`SceneComponent.K2_GetComponentLocation` (`self.CameraMesh`)) (`self.K2_GetActorLocation` (`self.DetectedActor`)) "TraceTypeQuery2"))
  (return _outhit _returnvalue))

(fn `FC_MoveOnActor`
  (bind _detectedactor (`self.DetectedActor`))
  (`/Engine/EditorBlueprintResources/StandardMacros.IsValid` _detectedactor
    (:`Is Valid`
      (if (and (<= (`self.GetDistanceTo` _detectedactor self) (`self.f_ChasingDistance`)) (`self.b_IsDetected`))
        (set `self.v3_TargetLocation` (`self.K2_GetActorLocation` (`self.DetectedActor`)))))))

(fn `FC_SetMainTrigger`
  (returns (OutHit :type "HitResult Structure") (IfCharacterDetected :type Boolean))
  (bind _v3_currentlocation (`self.v3_CurrentLocation`))
  (bind _returnvalue (`SceneComponent.K2_GetComponentLocation` (`self.CameraMesh`)))
  (bind (_outhit _returnvalue_2) (`KismetSystemLibrary.BoxTraceSingle` _returnvalue _v3_currentlocation (* (1.0 1.0 1.0) (`self.f_BoxSize`)) (`KismetMathLibrary.FindLookAtRotation` _returnvalue _v3_currentlocation) "TraceTypeQuery5"))
  (`self.FC_CameraLookAtOverlap`)
  (return _outhit _returnvalue_2))

(fn `UserConstructionScript`
  (`self.Refres_debug_box`))
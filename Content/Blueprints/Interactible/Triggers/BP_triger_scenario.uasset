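; BP_triger_scenario is a box trigger that activates its linked actors, typically a scenario manager, when the player enters.
; Overlap checks CanBeTrigered and the player cast, then fires CEForEachActorLink through a DoOnce, which Reset_triger_scenario re-arms.
; The TrigerOnce branch does the same either way, so it has no effect.
; The construction script labels its TextRender with the first linked scenario manager's ScenarioName.
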(event `self.Box.OnComponentBeginOverlap`
  (params (OverlappedComponent :type "PrimitiveComponent Object Reference") (OtherActor :type "Actor Object Reference") (OtherComp :type "PrimitiveComponent Object Reference") (OtherBodyIndex :type Integer) (bFromSweep :type Boolean) (SweepResult :type "HitResult Structure (by ref)"))
  (if (`self.CanBeTrigered`)
    (if (`self.TrigerOnce?`)
      _
      (else
        _))
    (cast `/Game/Blueprints/Characters/BP_PlayerCharacter` OtherActor)
    (`/Engine/EditorBlueprintResources/StandardMacros.DoOnce` false :!label _label
      (:`Completed`
        (`self.CE_ForEachActorLink` true)))))

(event `Reset_triger_scenario`
  (goto _label :!via `Reset`))

(fn `UserConstructionScript`
  (`parent.UserConstructionScript`)
  (bind _asbp_scenario_manager (cast `/Game/Blueprints/Interactible/Environments/BP_scenario_manager` (`|GetArrayItem` (`self.ActorLink`))))
  (`TextRenderComponent.K2_SetText` (`self.TextRender`) (`KismetTextLibrary.Conv_StringToText` (`/Game/Blueprints/Interactible/Environments/BP_scenario_manager.ScenarioName` _asbp_scenario_manager))))
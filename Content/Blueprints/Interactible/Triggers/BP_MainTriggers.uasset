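; BP_MainTriggers appears to be a base Blueprint for interactible triggers that act on linked actors.
; An EMP event raises an EMP flag and clears it after the supplied duration using a Delay.
; FC_ForEachActorLink writes the trigger's TriggerType into a linked actor's interaction struct, keeping its description and SFX.
; It returns from inside the loop, so only the first linked actor is updated.
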(event `self.ReceiveTick`
  (params (DeltaSeconds :type "Float (single-precision)"))
  (`parent.ReceiveTick` DeltaSeconds))

(event `/Game/Blueprints/Interactible/Items/Bullets/EMP/IEMP.EMP`
  (params (EMPDuration :type "Float (double-precision)"))
  (set `self.EMP?` true)
  (`KismetSystemLibrary.Delay` EMPDuration)
  (set `self.EMP?` false))

(fn `FC_ForEachActorLink`
  (returns (OutputPin :type "/Game/Blueprints/Interactible/Environments/BP_MainEnvironmentInteractible Object Reference"))
  (bind _actorlink (`self.ActorLink`))
  (if (`KismetArrayLibrary.Array_IsValidIndex` _actorlink)
    (for _array_element _actorlink
      (bind (_description _sfxs) (break `/Game/Blueprints/Interactible/Environments/S_EnvironmentInteractible` (`/Game/Blueprints/Interactible/Environments/BP_MainEnvironmentInteractible.S_ EnviroInteract` _array_element)))
      (set `/Game/Blueprints/Interactible/Environments/BP_MainEnvironmentInteractible.S_ EnviroInteract` (make `/Game/Blueprints/Interactible/Environments/S_EnvironmentInteractible` _description _sfxs (`self.TriggerType`)) _array_element)
      (return _array_element))))

(fn `UserConstructionScript`)
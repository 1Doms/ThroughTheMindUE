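; Blueprint function library of UI and localization helpers for the Through The Mind game.
; It looks up PDA colors, applies data-table font and shadow settings, and returns the cursor reference.
; Init and Close helpers message nested panel children through hand-unrolled loops four levels deep.
; Translations come from DT_Languages by enum-named row, choosing English or French from the language stored on the game instance.
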(fn `CloseAllchildsUI`
  (params (Object :type "PanelWidget Object Reference"))
  (for _array_element (`PanelWidget.GetAllChildren` Object)
    (message `/Game/UI/Widgets/IUpdateUI.Close` _array_element)
    (bind _aspanel_widget (cast `PanelWidget` _array_element))
    (for _array_element_2 (`PanelWidget.GetAllChildren` _aspanel_widget)
      (message `/Game/UI/Widgets/IUpdateUI.Close` _array_element_2)
      (bind _aspanel_widget_2 (cast `PanelWidget` _array_element_2))
      (for _array_element_3 (`PanelWidget.GetAllChildren` _aspanel_widget_2)
        (message `/Game/UI/Widgets/IUpdateUI.Close` _array_element_3)
        (bind _aspanel_widget_3 (cast `PanelWidget` _array_element_3))
        (for _array_element_4 (`PanelWidget.GetAllChildren` _aspanel_widget_3)
          (message `/Game/UI/Widgets/IUpdateUI.Close` _array_element_4))))))

(fn `Get cursor`
  (returns (Cursor_ref1 :type "/Game/UI/Widgets/Molecules/WBP_cursor Object Reference"))
  (locals (Cursor_ref :type "/Game/UI/Widgets/Molecules/WBP_cursor Object Reference"))
  (return (`local.Cursor_ref`)))

(fn `Get text settings`
  (params (RowName :type "/Game/UI/Font/EFontsName Enum" :default "NewEnumerator0"))
  (returns (`Text Settings` :type "/Game/UI/Font/F_Fonts Structure"))
  (locals (DT_text :type "DataTable Object Reference" :default "/Script/Engine.DataTable'/Game/UI/Font/DT_Text.DT_Text'"))
  (bind _returnvalue (`|GetDataTableRow` (`local.DT_text`) (`KismetStringLibrary.Conv_StringToName` (`|GetEnumeratorNameAsString` RowName)))
    (:`then`
      (return _returnvalue))))

(fn `Get UI color`
  (params (Name :type "/Game/UI/Colors/EColors Enum" :default "NewEnumerator0"))
  (returns (Color :type "LinearColor Structure"))
  (locals (PDA_colors :type "/Game/UI/Colors/PDA_colors Object Reference" :default "/Game/UI/Colors/PDA_colors.PDA_colors_C'/Game/UI/Colors/DA_colors.DA_colors'"))
  (return (`BlueprintMapLibrary.Map_Find` (`/Game/UI/Colors/PDA_colors.Colors` (`local.PDA_colors`)) Name)))

(fn `GetGameInstance`
  (returns (`AsBP Through the Mind GI` :type "/Game/Blueprints/BP_ThroughTheMind_GI Object Reference"))
  (bind _asbp_through_the_mind_gi (cast `/Game/Blueprints/BP_ThroughTheMind_GI` (`GameplayStatics.GetGameInstance` null)))
  (return _asbp_through_the_mind_gi))

(fn `GetLanguage`
  (returns (Language :type "/Game/UI/Languages/Elanguages Enum"))
  (return (`/Game/Blueprints/BP_ThroughTheMind_GI.Language` (`self.GetGameInstance` null))))

(fn `GetLanguageText`
  (params (TextType :type "/Game/UI/Languages/ElanguagesTexts Enum" :default "NewEnumerator0"))
  (returns (Text :type Text))
  (bind _returnvalue (`|GetDataTableRow` "/Game/UI/Languages/DT_Languages.DT_Languages" (`KismetStringLibrary.Conv_StringToName` (`|GetEnumeratorNameAsString` TextType)))
    (:`then`
      (switch `/Game/UI/Languages/Elanguages` (`self.GetLanguage` null)
        (:`NewEnumerator0`
          (bind (_englishtext _frenchtext) (break `/Game/UI/Languages/F_Languages` _returnvalue))
          (return _englishtext))
        (:`NewEnumerator1`
          (return _frenchtext))))
    (:`RowNotFound`
      (return "No translation"))))

(fn `InitAllchildsUI`
  (params (Target :type "PanelWidget Object Reference"))
  (for _array_element (`PanelWidget.GetAllChildren` Target)
    (message `/Game/UI/Widgets/IUpdateUI.Init` _array_element)
    (bind _aspanel_widget (cast `PanelWidget` _array_element))
    (for _array_element_2 (`PanelWidget.GetAllChildren` _aspanel_widget)
      (message `/Game/UI/Widgets/IUpdateUI.Init` _array_element_2)
      (bind _aspanel_widget_2 (cast `PanelWidget` _array_element_2))
      (for _array_element_3 (`PanelWidget.GetAllChildren` _aspanel_widget_2)
        (message `/Game/UI/Widgets/IUpdateUI.Init` _array_element_3)
        (bind _aspanel_widget_3 (cast `PanelWidget` _array_element_3))
        (for _array_element_4 (`PanelWidget.GetAllChildren` _aspanel_widget_3)
          (message `/Game/UI/Widgets/IUpdateUI.Init` _array_element_4))))))

(fn `Set text settings`
  (params (Object :type "TextBlock Object Reference") (RowName :type "/Game/UI/Font/EFontsName Enum" :default "NewEnumerator0"))
  (bind (_name _style _size _shadowcolor) (break `/Game/UI/Font/F_Fonts` (`self.Get text settings` RowName)))
  (`TextBlock.SetFont` Object (make `SlateFontInfo` _style null (struct :`OutlineColor` (struct :`A` 1.0)) "None" _size))
  (`TextBlock.SetShadowColorAndOpacity` Object (`KismetMathLibrary.Conv_ColorToLinearColor` _shadowcolor)))

(fn `SetLanguage`
  (params (Language :type "/Game/UI/Languages/Elanguages Enum" :default "NewEnumerator0"))
  (set `/Game/Blueprints/BP_ThroughTheMind_GI.Language` Language (`self.GetGameInstance` null)))
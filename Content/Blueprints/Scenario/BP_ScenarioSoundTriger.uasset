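; BP_ScenarioSoundTriger is a scenario trigger volume that plays a positioned sound after the player enters it.
; The first overlap by BP_PlayerCharacter passes a DoOnce and sets a timer with a random delay between Min and Max, optionally looping.
; The timer plays the configured sound at the actor's location plus an offset, with configurable volume and attenuation.
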(event `self.Box.OnComponentBeginOverlap`
  (params (OverlappedComponent :type "PrimitiveComponent Object Reference") (OtherActor :type "Actor Object Reference") (OtherComp :type "PrimitiveComponent Object Reference") (OtherBodyIndex :type Integer) (bFromSweep :type Boolean) (SweepResult :type "HitResult Structure (by ref)"))
  (cast `/Game/Blueprints/Characters/BP_PlayerCharacter` OtherActor)
  (`/Engine/EditorBlueprintResources/StandardMacros.DoOnce` false
    (:`Completed`
      (`KismetSystemLibrary.K2_SetTimerDelegate` (delegate `PlaySound`) (`KismetMathLibrary.RandomFloatInRange` (`self.Min`) (`self.Max`)) (`self.Looping`)))))

(event `PlaySound`
  (`GameplayStatics.PlaySoundAtLocation` (`self.Sound`) (+ (`self.K2_GetActorLocation`) (`self.SoundPosition`)) (struct) (`self.Volume Multiplier`) 1.0 0.0 (`self.Attenuation Settings`) null null null))

(fn `UserConstructionScript`)
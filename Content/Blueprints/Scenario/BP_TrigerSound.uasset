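; One-shot scenario trigger that plays a sound when the player character overlaps its box or when it receives an Activated event.
; The sound plays either as 2D or at the SoundLocation component with attenuation settings.
; It can optionally wait, then send Activated messages to a list of other actors to chain events.
; The actor destroys itself afterwards.
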(event `/Game/Blueprints/Interactible/BPI_Interaction.Activated`
  (bind _sound (`self.Sound`))
  (if (`self.2D_Sound?`) :!label _label
    (`GameplayStatics.PlaySound2D` _sound 1.0 1.0 0.0 null null)
    (else
      (`GameplayStatics.PlaySoundAtLocation` _sound (`SceneComponent.K2_GetComponentLocation` (`self.SoundLocation`)) (struct) 1.0 1.0 0.0 (`self.Attenuation Settings`) null null null)))
  (if (`self.ShouldTrigerActor?`)
    (`KismetSystemLibrary.Delay` (`self.DelayBeforeActivatedAnotherActor`))
    (for _array_element (`self.ActorToTriger`)
      (message `/Game/Blueprints/Interactible/BPI_Interaction.Activated` _array_element)))
  (`self.K2_DestroyActor`))

(event `self.Box.OnComponentBeginOverlap`
  (params (OverlappedComponent :type "PrimitiveComponent Object Reference") (OtherActor :type "Actor Object Reference") (OtherComp :type "PrimitiveComponent Object Reference") (OtherBodyIndex :type Integer) (bFromSweep :type Boolean) (SweepResult :type "HitResult Structure (by ref)"))
  (cast `/Game/Blueprints/Characters/BP_PlayerCharacter` OtherActor)
  (goto _label))

(fn `UserConstructionScript`)
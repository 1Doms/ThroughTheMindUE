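; One-shot scripted encounter trigger that stages an Alpha AI appearance when the player enters its box.
; The first overlap consumes the DoOnce before the player cast, then DoorToActivated fires twice, one second apart.
; Meanwhile the Alpha teleports to the TP point and, after a short delay, a looping timer repeatedly targets it at the player's current location.
; After several seconds the timer is cleared and the trigger destroys itself.
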(event `self.ReceiveActorBeginOverlap`
  (params (OtherActor :type "Actor Object Reference")))

(event `self.Box.OnComponentBeginOverlap`
  (params (OverlappedComponent :type "PrimitiveComponent Object Reference") (OtherActor :type "Actor Object Reference") (OtherComp :type "PrimitiveComponent Object Reference") (OtherBodyIndex :type Integer) (bFromSweep :type Boolean) (SweepResult :type "HitResult Structure (by ref)"))
  (`/Engine/EditorBlueprintResources/StandardMacros.DoOnce` false
    (:`Completed`
      (cast `/Game/Blueprints/Characters/BP_PlayerCharacter` OtherActor)
      (`/Game/Blueprints/Interactible/BPI_Interaction.Activated` (`self.DoorToActivated`))
      (`|ExecutionSequence`
        (:`then_0`
          (`KismetSystemLibrary.Delay` 1.0)
          (`/Game/Blueprints/Interactible/BPI_Interaction.Activated` (`self.DoorToActivated`)))
        (:`then_1`
          (bind _returnvalue (`GameplayStatics.GetActorOfClass` "/Game/Blueprints/AI/Blueprints/BP_AI_character_alpha.BP_AI_character_alpha_C"))
          (`self.K2_SetActorLocation` _returnvalue (`SceneComponent.K2_GetComponentLocation` (`self.TP`)) false false)
          (`KismetSystemLibrary.Delay` 1.0)
          (bind _returnvalue_2 (`KismetSystemLibrary.K2_SetTimerDelegate` (delegate `PingPlayer`) 0.1 true))
          (`KismetSystemLibrary.Delay` 5.0)
          (`KismetSystemLibrary.K2_ClearAndInvalidateTimerHandle` _returnvalue_2)
          (`self.K2_DestroyActor`))))))

(event `PingPlayer`
  (bind _returnvalue (`GameplayStatics.GetActorOfClass` "/Game/Blueprints/Characters/BP_PlayerCharacter.BP_PlayerCharacter_C"))
  (bind _returnvalue_2 (`GameplayStatics.GetActorOfClass` "/Game/Blueprints/AI/Blueprints/BP_AI_character_alpha.BP_AI_character_alpha_C"))
  (`/Game/Blueprints/AI/Blueprints/BP_AI_character.Target_set` _returnvalue_2 _returnvalue (`self.K2_GetActorLocation` _returnvalue)))

(fn `UserConstructionScript`)
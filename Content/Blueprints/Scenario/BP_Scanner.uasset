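; BP_Scanner is a scenario scanner actor that, once activated, turns its Sphere component to follow the player.
; It finds BP_PlayerCharacter at BeginPlay, and Activated reveals the NSScanner effect.
; A looping timer set to the frame delta stands in for Tick, smoothly interpolating the sphere's rotation toward the player.
; Desactived clears that timer and destroys the actor.
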(event `self.ReceiveBeginPlay`
  (bind _returnvalue (`GameplayStatics.GetActorOfClass` "/Game/Blueprints/Characters/BP_PlayerCharacter.BP_PlayerCharacter_C"))
  (set `self.PlayerRef` _returnvalue))

(event `/Game/Blueprints/Interactible/BPI_Interaction.Activated`
  (`SceneComponent.SetHiddenInGame` (`self.NS_Scanner`) false false)
  (bind _returnvalue (`KismetSystemLibrary.K2_SetTimerDelegate` (delegate `LookAt`) (`GameplayStatics.GetWorldDeltaSeconds`) true)))

(event `LookAt`
  (bind _sphere (`self.Sphere`))
  (`SceneComponent.K2_SetWorldRotation` _sphere (`KismetMathLibrary.RInterpTo` (`SceneComponent.K2_GetComponentRotation` _sphere) (`KismetMathLibrary.FindLookAtRotation` (`SceneComponent.K2_GetComponentLocation` _sphere) (`self.K2_GetActorLocation` (`self.PlayerRef`))) (`GameplayStatics.GetWorldDeltaSeconds`) 2.0) false false))

(event `/Game/Blueprints/Interactible/BPI_Interaction.Desactived`
  (`KismetSystemLibrary.K2_ClearAndInvalidateTimerHandle` (stale `/Game/Blueprints/Interactible/BPI_Interaction.Activated` _returnvalue))
  (`SceneComponent.SetHiddenInGame` (`self.NS_Scanner`) false false)
  (`self.K2_DestroyActor`))

(fn `UserConstructionScript`)
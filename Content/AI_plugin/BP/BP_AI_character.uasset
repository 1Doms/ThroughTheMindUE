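; Base AI character that picks a target among perceived actors using a detection score and scales its walk speed to that score.
; AI Perception updates maintain parallel arrays of detected actors and scores.
; Each tick, scores combine distance, offset from facing and brightness difference from a light-detection child actor; the highest above a threshold becomes the target.
; Empty events for sensing, targeting, roaming radius and tick serve as hooks, with debug prints throughout.
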(event `Succesfull_sensed`)

(event `self.AIPerception.OnPerceptionUpdated`
  (params (UpdatedActors :type "Array of Actor Object Reference (by ref)"))
  (bind _target (`self.Target`))
  (bind _array_of_actors_detected (`self.Array_of_actors_detected`))
  ;[1 1 1] get all actor seen
  (for _array_element UpdatedActors
    (bind _info (`AIPerceptionComponent.GetActorsPerception` (`self.AIPerception`) _array_element))
    (bind (_target_2 _lastsensedstimuli) (break `ActorPerceptionBlueprintInfo` _info))
    (set `self.Target` _target_2)
    (for _array_element_2 _lastsensedstimuli
      (if (`.bSuccessfullySensed` (break `AIStimulus` _array_element_2))
        (`KismetArrayLibrary.Array_Add` _array_of_actors_detected _target)
        (`KismetArrayLibrary.Array_Add` (`self.Array_of_detection_score`))
        ;[0.9743 0 1] Debug
        (`KismetSystemLibrary.PrintString` (`KismetSystemLibrary.GetDisplayName` _target) true false (struct :`G` 1.0 :`B` 0.006319 :`A` 1.0) 1.0)
        (`self.Succesfull_sensed`)
        (else
          (`KismetArrayLibrary.Array_RemoveItem` _array_of_actors_detected _target)
          (`KismetArrayLibrary.Array_Remove` (`self.Array_of_detection_score`) (+ (`KismetArrayLibrary.Array_Find` _array_of_actors_detected _target) 1))
          (`KismetSystemLibrary.PrintString` (`KismetSystemLibrary.GetDisplayName` _target) true false (struct :`R` 1.0 :`B` 0.095176 :`A` 1.0) 1.0)
          (`self.Not_sensed`))))))

(event `Not_sensed`)

(event `Set_Roaming_Raddius`)

(event `self.ReceiveBeginPlay`
  (`self.Set_Roaming_Raddius`))

(event `self.ReceiveTick`
  (params (DeltaSeconds :type "Float (single-precision)"))
  (bind _array_of_actors_detected (`self.Array_of_actors_detected`))
  (bind (_indexofmaxvalue _maxvalue) (`KismetMathLibrary.MaxOfFloatArray` (`self.Array_of_detection_score`)))
  (`self.Tick_child` DeltaSeconds)
  (`self.Modify_Speed`)
  (`KismetSystemLibrary.DelayUntilNextTick`)
  (bind _asbp_light_detection (cast `/Game/AI_plugin/BP/BP_LightDetection` (`ChildActorComponent.ChildActor` (`self.BP_LightDetection`))))
  (set `self.Self_brightness` (`/Game/AI_plugin/BP/BP_LightDetection.BP_LightDetection_Brightness` _asbp_light_detection))
  (if (not (`KismetArrayLibrary.Array_IsEmpty` _array_of_actors_detected))
    (for (_array_element _array_index) _array_of_actors_detected
      (`self.Calcul_detection_score` _array_element _array_index))
    (if (> _maxvalue 0.2)
      (bind _output_get (set `self.Choosen_target` (`|GetArrayItem` (`self.Array_of_actors_detected`) _indexofmaxvalue)))
      (`KismetSystemLibrary.PrintString` (`KismetSystemLibrary.GetDisplayName` _output_get) true false (struct :`R` 0.117799 :`B` 1.0 :`A` 1.0) 0.0)
      (`self.Target_set` _output_get (`self.K2_GetActorLocation` _output_get))
      (else
        (set `self.Choosen_target` null)))))

(event `Target_set`
  (params (Target_ref :type "Actor Object Reference") (Target_Location :type "Vector Structure")))

(event `Tick_child`
  (params (Delta_seconds :type "Float (double-precision)")))

(event `Modify_Speed`
  (bind _min_speed (`self.Min_Speed`))
  (bind _charactermovement (`self.CharacterMovement`))
  (`KismetSystemLibrary.PrintString` (`KismetStringLibrary.Conv_DoubleToString` (`CharacterMovementComponent.MaxWalkSpeed` (`self.CharacterMovement`))) true false (struct :`G` 0.66 :`B` 1.0 :`A` 1.0) 0.0)
  (if (`KismetSystemLibrary.IsValid` (`self.Choosen_target`))
    (set `CharacterMovementComponent.MaxWalkSpeed` (`KismetMathLibrary.MapRangeClamped` (`.MaxValue` (`KismetMathLibrary.MaxOfFloatArray` (`self.Array_of_detection_score`))) 0.0 1.0 _min_speed (`self.Max_Speed`)) _charactermovement)
    (else
      (set `CharacterMovementComponent.MaxWalkSpeed` _min_speed _charactermovement))))

(fn `Angle_between_two_vectors`
  (params (`Vector 1` :type "Vector Structure") (`Vector 2` :type "Vector Structure"))
  (returns (Angle :type "Float (double-precision)"))
  (return (`KismetMathLibrary.DegAcos` (`KismetMathLibrary.Dot_VectorVector` (`KismetMathLibrary.Normal` `Vector 1`) (`KismetMathLibrary.Normal` `Vector 2`)))))

(fn `UserConstructionScript`)
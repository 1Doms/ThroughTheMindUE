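; Tentacle actor that stretches a Niagara effect from itself to a traced surface point while following its owner.
; On BeginPlay a randomized narrow-cone line trace picks the anchor, and the actor destroys itself if nothing is hit.
; Each Tick it re-snaps to its owner and updates the effect's start point.
; Exceeding the maximum distance from the anchor destroys the effect, then the actor if the effect reports being destroyed.
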(event `self.ReceiveBeginPlay`
  (bind _returnvalue (`self.K2_GetActorLocation`))
  (bind _tantacle_ref (`self.Tantacle_ref`))
  (bind (_outhit _returnvalue_2) (`KismetSystemLibrary.LineTraceSingle` :`Start` _returnvalue :`End` (* (`KismetMathLibrary.RandomUnitVectorInConeInDegrees` (+ (`SceneComponent.GetForwardVector` (`self.DefaultSceneRoot`)) (`self.K2_GetActorLocation`)) 5.0) (`self.Tantacle_max_distance`)) :`TraceChannel` "TraceTypeQuery1" :`DrawDebugType` "ForDuration" :`DrawTime` 2.0))
  (if _returnvalue_2
    (bind _returnvalue_3 (`NiagaraFunctionLibrary.SpawnSystemAtLocation` (`self.Tantacle_system`) _returnvalue (struct) (1.0 1.0 1.0) false))
    (set `self.Tantacle_ref` _returnvalue_3)
    (`FXSystemComponent.SetVectorParameter` _tantacle_ref "Tantacle_Start" _returnvalue)
    (bind (_bblockinghit _binitialoverlap _time _distance _location) (`GameplayStatics.BreakHitResult` _outhit))
    (`FXSystemComponent.SetVectorParameter` _tantacle_ref "Tantacle_End" _location)
    (set `self.End_location` _location)
    (set `self.Tantacle_exist` true)
    (else
      (`self.K2_DestroyActor`))))

(event `self.ReceiveTick`
  (params (DeltaSeconds :type "Float (single-precision)"))
  (bind _returnvalue (`self.GetOwner`))
  (bind _tantacle_ref (`self.Tantacle_ref`))
  (`KismetSystemLibrary.PrintString` (`KismetSystemLibrary.GetDisplayName` _returnvalue) true true (struct :`G` 1.0 :`B` 0.447227 :`A` 1.0) 0.0)
  (`self.K2_AttachToActor` _returnvalue "None" "SnapToTarget" "SnapToTarget" "KeepRelative")
  (if (`self.Tantacle_exist`)
    (`FXSystemComponent.SetVectorParameter` (`self.Tantacle_ref`) "Tantacle_Start" (`self.K2_GetActorLocation`))
    (if (> (`KismetMathLibrary.Vector_Distance` (`self.End_location`) (`self.K2_GetActorLocation`)) (`self.Tantacle_max_distance`))
      (`ActorComponent.K2_DestroyComponent` _tantacle_ref)
      (if (`ActorComponent.IsBeingDestroyed` _tantacle_ref)
        (`self.K2_DestroyActor`)))))

(fn `UserConstructionScript`)
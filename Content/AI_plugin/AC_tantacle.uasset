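; AC_tantacle is an actor component that spawns BP_tantacle actors at its owning Character's transform while the character moves.
; Each Tick, it compares the last index of a GetAllActorsOfClass loop against MaxNumberOfTantacle to cap spawning.
; If velocity exceeds a small threshold, it waits a random SpawnRate delay, then spawns a tentacle owned by the character.
; Debug prints report movement state and missing Character or movement component.
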(event `self.ReceiveBeginPlay`
  (set `self.Tantacle_actor` "/Game/AI_plugin/BP_tantacle.BP_tantacle_C"))

(event `self.ReceiveTick`
  (params (DeltaSeconds :type "Float (single-precision)"))
  (bind _returnvalue (`self.GetOwner`))
  (bind (_spawn_rate_x _spawn_rate_y) (`KismetMathLibrary.BreakVector2D` (`self.Spawn_rate`)))
  (bind (_returnvalue_location _returnvalue_rotation) (`KismetMathLibrary.BreakTransform` (`Actor.GetTransform` (`self.GetOwner`))))
  (bind _outactors (`GameplayStatics.GetAllActorsOfClass` null))
  (for (_ _array_index) _outactors
    _)
  (if (not (> _array_index (`self.Max_number_of_tantacle`)))
    (bind _ascharacter (cast `Character` _returnvalue)
      (:`then`
        (bind _charactermovement (`Character.CharacterMovement` _ascharacter))
        (`/Engine/EditorBlueprintResources/StandardMacros.IsValid` _charactermovement
          (:`Is Valid`
            (if (> (`KismetMathLibrary.VSize` (`MovementComponent.Velocity` _charactermovement)) 25.0)
              (`KismetSystemLibrary.PrintString` "Moving" true true (struct :`R` 0.653681 :`B` 1.0 :`A` 1.0) 0.1)
              (`KismetSystemLibrary.Delay` (`KismetMathLibrary.RandomFloatInRange` _spawn_rate_x _spawn_rate_y))
              (`|SpawnActorFromClass` (`self.Tantacle_actor`) (`KismetMathLibrary.MakeTransform` _returnvalue_location _returnvalue_rotation) "AlwaysSpawn" "MultiplyWithRoot" _returnvalue null)
              (else
                (`KismetSystemLibrary.PrintString` "Not moving" true true (struct :`R` 0.653681 :`B` 1.0 :`A` 1.0) 0.1))))
          (:`Is Not Valid`
            (`KismetSystemLibrary.PrintString` "There is no character movement for the owner of AC_tantacle" true true (struct :`R` 1.0 :`B` 0.525952 :`A` 1.0)))))
      (:`CastFailed`
        (`KismetSystemLibrary.PrintString` "There is no character for the owner of AC_tantacle" true true (struct :`R` 1.0 :`B` 0.525952 :`A` 1.0))))))
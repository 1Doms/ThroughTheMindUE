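; Actor component that measures how lit its owner is and exposes it as a normalized Brightness value.
; On BeginPlay it gives the owner's child SceneCaptureComponent2D its own render target, sized like the assigned one.
; Each tick it reads that target's center pixel and computes weighted RGB luminance, then rounds, clamps and divides by MaxClamp.
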(event `self.ReceiveBeginPlay`
  ;[1 1 1] Find RT_Text
  (bind _asscene_capture_component_2d (cast `SceneCaptureComponent2D` (`SceneComponent.GetChildComponent` (`Actor.RootComponent` (`self.GetOwner`)) 0)))
  (bind _texturetarget (`SceneCaptureComponent2D.TextureTarget` _asscene_capture_component_2d))
  ;[1 1 1] Create a new render target 2D with same properties than RT_text and asign it the the owner scene component
  (bind _returnvalue (`KismetRenderingLibrary.CreateRenderTarget2D` (`TextureRenderTarget2D.SizeX` _texturetarget) (`TextureRenderTarget2D.SizeY` _texturetarget) "RTF_RGBA16f" (struct :`A` 1.0) true))
  (bind _output_get (set `SceneCaptureComponent2D.TextureTarget` _returnvalue _asscene_capture_component_2d))
  (set `self.Current_render_texture` _output_get))

(event `self.ReceiveTick`
  (params (DeltaSeconds :type "Float (single-precision)"))
  (bind _current_render_texture (`self.Current_render_texture`))
  (bind _max_clamp (`self.Max_clamp`))
  ;[1 1 1] Update brightness value
  (`KismetSystemLibrary.DelayUntilNextTick`)
  ;;[1 1 1] Get middle pixel
  (bind _returnvalue (`KismetRenderingLibrary.ReadRenderTargetPixel` (`self.Current_render_texture`) (/ (`TextureRenderTarget2D.SizeX` _current_render_texture) 2) (/ (`TextureRenderTarget2D.SizeY` _current_render_texture) 2)))
  ;;[1 1 1] Calc light intensity
  (bind _output_get (set `self.Texture_brightness` (+ (* (`KismetMathLibrary.Conv_ByteToDouble` (break `Color` _returnvalue)) 0.0722) (+ (* (`KismetMathLibrary.Conv_ByteToDouble` (`.G` (break `Color` _returnvalue))) 0.7152) (* (`KismetMathLibrary.Conv_ByteToDouble` (`.R` (break `Color` _returnvalue))) 0.2126)))))
  (set `self.Brightness` (/ (`KismetMathLibrary.FClamp` (`KismetMathLibrary.Conv_IntToDouble` (`KismetMathLibrary.Round` _output_get)) 0.0 _max_clamp) _max_clamp)))
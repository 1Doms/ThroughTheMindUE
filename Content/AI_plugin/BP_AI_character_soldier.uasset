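; BP_AI_character_soldier is an AI soldier character that passes perception results and roaming settings to the BB_alpha blackboard.
; Sensing events set the target flag, clearing it only once the detected-actors array is empty.
; Other events write the target reference, target location and roaming radius to their keys.
; The BeginPlay, overlap, Tick stubs are disabled, and the construction script only calls its parent.
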(event `self.Succesfull_sensed`
  ;[0.007497 0 1] Modify key variables of BB_alpha
  (`BlackboardComponent.SetValueAsBool` (`AIBlueprintHelperLibrary.GetBlackboard` null) "Target?" true))

(event `self.Not_sensed`
  ;[0.007497 0 1] Modify key variables of BB_alpha
  (if (`KismetArrayLibrary.Array_IsEmpty` (`self.Array_of_actors_detected`))
    (`BlackboardComponent.SetValueAsBool` (`AIBlueprintHelperLibrary.GetBlackboard` null) "Target?" false)))

(event `self.Target_set`
  (params (Target_ref :type "Actor Object Reference") (Target_Location :type "Vector Structure"))
  (bind _returnvalue (`AIBlueprintHelperLibrary.GetBlackboard` null))
  ;[0.007497 0 1] Modify key variables of BB_alpha
  (`BlackboardComponent.SetValueAsObject` _returnvalue "Target_reference" Target_ref)
  (`BlackboardComponent.SetValueAsVector` _returnvalue "Target_Location" Target_Location))

(event `self.Set_Roaming_Raddius`
  ;[0.007497 0 1] Modify key variables of BB_alpha
  (`BlackboardComponent.SetValueAsFloat` (`AIBlueprintHelperLibrary.GetBlackboard` null) "Roaming_Radius" (`self.Roaming_radius`)))

(fn `UserConstructionScript`
  (`parent.UserConstructionScript`))
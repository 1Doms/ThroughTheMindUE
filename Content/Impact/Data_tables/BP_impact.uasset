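; BP_impact is an impact effect actor that plays surface-specific sound, decal and particles at a hit point.
; On BeginPlay it unpacks its Hit and looks up the DT_impact row named after the physical surface type.
; Its Name selects that row's entry for Soldier Gun or Soldier Step; a third entry is unwired.
; Effects are chained: the randomly sized, attached decal requires a valid sound, and the Niagara particles require a valid decal.
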(event `self.ReceiveBeginPlay`
  (bind (_bblockinghit _binitialoverlap _time _distance _location _impactpoint _normal _impactnormal _physmat _hitactor _hitcomponent _hitbonename) (`GameplayStatics.BreakHitResult` (`self.Hit`)))
  (set `self.Location` _location)
  (set `self.Impact Point` _impactpoint)
  (set `self.Surface Type` (`PhysicalMaterial.SurfaceType` _physmat))
  (set `self.Hit Actor` _hitactor)
  (set `self.Hit Component` _hitcomponent)
  (set `self.Hit Bone Name` _hitbonename)
  (bind _returnvalue (`|GetDataTableRow` "/Game/Impact/Data_tables/DT_impact.DT_impact" (`KismetStringLibrary.Conv_StringToName` (`|GetEnumeratorNameAsString` (`self.Surface Type`))))
    (:`then`
      (set `self.Out Row` _returnvalue)
      (`self.Check_origin`))))

(event `Check_origin`
  (bind _dt_impact (break `/Game/Impact/Data_tables/F_DT_impact` (`self.Out Row`)))
  (switch `/Game/Impact/Data_tables/E_Name` (`self.Name`)
    (:`NewEnumerator0`
      (`self.Execute_impact_data_table` (`|GetArrayItem` _dt_impact)))
    (:`NewEnumerator3`
      (`self.Execute_impact_data_table` (`|GetArrayItem` _dt_impact 1)))))

(fn `Execute_impact_data_table`
  (params (NewParam :type "/Game/Impact/Data_tables/F_impact_data Structure"))
  (bind (_surface _name _impact_sound _impact_decal _decal_min_size _decal_max_size _impact_particle) (break `/Game/Impact/Data_tables/F_impact_data` NewParam))
  (bind (_x _y _z) (`KismetMathLibrary.BreakVector3f` _decal_max_size))
  (bind (_x_2 _y_2 _z_2) (`KismetMathLibrary.BreakVector3f` _decal_min_size))
  (`/Engine/EditorBlueprintResources/StandardMacros.IsValid` _impact_sound
    (:`Is Valid`
      (`GameplayStatics.SpawnSoundAtLocation` _impact_sound (`self.Impact Point`) (struct) 1.0 1.0 0.0 "/Game/Sounds/Sounds/SA_test.SA_test" null)
      (`/Engine/EditorBlueprintResources/StandardMacros.IsValid` _impact_decal
        (:`Is Valid`
          (`GameplayStatics.SpawnDecalAttached` _impact_decal (`KismetMathLibrary.MakeVector` (`KismetMathLibrary.RandomFloatInRange` _x_2 _x) (`KismetMathLibrary.RandomFloatInRange` _y_2 _y) (`KismetMathLibrary.RandomFloatInRange` _z_2 _z)) (`self.Hit Component`) (`self.Hit Bone Name`) (`self.Impact Point`) (struct) "SnapToTarget")
          (for _array_element _impact_particle
            (`/Engine/EditorBlueprintResources/StandardMacros.IsValid` _array_element
              (:`Is Valid`
                (`NiagaraFunctionLibrary.SpawnSystemAtLocation` _array_element (`self.Impact Point`))))))))))

(fn `UserConstructionScript`)
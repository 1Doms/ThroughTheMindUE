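; BP_Sas is a level actor that streams in a set of levels at BeginPlay, then activates a linked interactible.
; A manual counter loop loads each soft-referenced level visible and blocking.
; Once loading calls finish, it calls Activated on the actor returned by the ActorLink helper.
; That helper rebuilds the environment-interact struct with this actor's TriggerType, returning from inside the loop at the first element.
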(event `self.ReceiveBeginPlay`
  (set `self.LoopCounter` 0)
  (set `self.ArrayIndex` 0)
  (if (< (`self.LoopCounter`) (`KismetArrayLibrary.Array_Length` (`self.Level`))) :!label _label
    (set `self.ArrayIndex` (`self.LoopCounter`))
    (`GameplayStatics.LoadStreamLevelBySoftObjectPtr` (`|GetArrayItem` (`self.Level`) (`self.ArrayIndex`)) true true)
    (set `self.LoopCounter` (+ (`self.LoopCounter`) 1))
    (goto _label)
    (else
      (bind _outputpin (`self.FC_ForEachActorLink`))
      (`/Game/Blueprints/Interactible/BPI_Interaction.Activated` _outputpin))))

(fn `FC_ForEachActorLink_0`
  (returns (`Array Element` :type "/Game/Blueprints/Interactible/Environments/BP_MainEnvironmentInteractible Object Reference"))
  (bind _actorlink (`self.ActorLink`))
  (if (`KismetArrayLibrary.Array_IsValidIndex` _actorlink)
    (for _array_element _actorlink
      (bind (_description _sfxs) (break `/Game/Blueprints/Interactible/Environments/S_EnvironmentInteractible` (`/Game/Blueprints/Interactible/Environments/BP_MainEnvironmentInteractible.S_ EnviroInteract` _array_element)))
      (set `/Game/Blueprints/Interactible/Environments/BP_MainEnvironmentInteractible.S_ EnviroInteract` (make `/Game/Blueprints/Interactible/Environments/S_EnvironmentInteractible` _description _sfxs (`self.TriggerType`)) _array_element)
      (return _array_element))))

(fn `UserConstructionScript`
  (`parent.UserConstructionScript`))
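; BP_Modular is a modular environment Blueprint that builds a flat grid of copies of one mesh.
; Its construction script looks up the Item data table row and, if found, assigns that row's static mesh to an Instanced Static Mesh component.
; Nested loops over the X and Y count variables add unscaled local-space instances, with the scale variables setting only the spacing.
; The event graph holds only disabled default events.
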(fn `UserConstructionScript`
  (bind (_datatable _rowname) (break `DataTableRowHandle` (`self.Item`)))
  (`parent.UserConstructionScript`)
  (bind _returnvalue (`|GetDataTableRow` _datatable _rowname)
    (:`then`
      (`StaticMeshComponent.SetStaticMesh` (`self.InstancedStaticMesh`) (`.StaticMesh_5_70B491EF4F7DDAA385D3E5A0FF2D5272` (break `/Game/Environments/Enum/S_EnvironmentProps` _returnvalue)))
      (for _index (range (+ (- (`self.X_NumInst`) 0) 1))
        (for _index_2 (range (+ (- (`self.Y_NumInst`) 0) 1))
          (`InstancedStaticMeshComponent.AddInstance` (`self.InstancedStaticMesh`) (`KismetMathLibrary.MakeTransform` (`KismetMathLibrary.MakeVector` (`KismetMathLibrary.Conv_IntToDouble` (* _index (* (`self.X_Scale`) 128))) (`KismetMathLibrary.Conv_IntToDouble` (* _index_2 (* (`self.Y_Scale`) 128))))) false))))))